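; Gold pickup actor that awards its gold amount to the player who picks it up.
; On the pickup event, an IsBeingPicked flag guards against repeat collection.
; It spawns a PickupOnWorld actor at the player's location to show the amount, calls PickupGold on the player, then destroys itself.
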(event `self.PickedUpByPlayer`
  (params (PlayerRef :type "/Game/Blueprints/HeroCartPlayer/PlayerCart Object Reference"))
  (bind _goldamount (`self.GoldAmount`))
  ;[1 1 1] Spawn Gold pickup widget
  (if (not (`self.IsBeingPicked`))
    (set `self.IsBeingPicked` true)
    (`|SpawnActorFromClass` "/Game/Blueprints/UI/PickupOnWorld.PickupOnWorld_C" (`KismetMathLibrary.Conv_VectorToTransform` (`self.K2_GetActorLocation` PlayerRef)) "AlwaysSpawn" "OverrideRootScale" null _goldamount (1.0 0.9 0.0) "NewEnumerator0" null)
    ;[1 1 1] Give gold to player
    (`/Game/Blueprints/HeroCartPlayer/PlayerCart.PickupGold` PlayerRef _goldamount)
    (`self.K2_DestroyActor`)))

(fn `UserConstructionScript`
  (`parent.UserConstructionScript`))