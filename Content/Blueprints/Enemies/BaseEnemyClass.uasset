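; Base enemy for HeroCart that scales health by level, registers with the game instance and handles damage and death.
; TakeDamage sums the damage entries, displays the number through the game mode and, without a current target, moves a surviving enemy toward its attacker.
; Lethal hits ragdoll the mesh, drop random gold and unregister the enemy.
; Tick destroys enemies behind the WallOfDeathX material parameter collection value, skipping loot and unregistration.
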(event `self.ReceiveTick`
  (params (DeltaSeconds :type "Float (single-precision)"))
  ;[1 0 0.04473 0.813] Killed by wall of death
  (if (`self.IsAlive`)
    (bind _returnvalue (`KismetMaterialLibrary.GetScalarParameterValue` "/Game/VFX/PostProcess/PostProcessGlobalParameters.PostProcessGlobalParameters" "WallOfDeathX"))
    (if (<= (.x (`self.K2_GetActorLocation`)) _returnvalue)
      (set `self.IsAlive` false)
      (`self.K2_DestroyActor`))))

(event `self.ReceiveBeginPlay`
  ;[0.2538 1 0 0.635] SetMaxHealth
  (bind _output_get (set `self.MaxHealth` (* (`self.MaxHealthPerLevel`) (`self.Level`))))
  (set `self.CurrentHealth` _output_get)
  ;[1 0.2417 0.9092 0.396] Add enemy to master list on game instance
  (bind _ashcgame_instance (cast `/Game/Blueprints/HCGameInstance` (`GameplayStatics.GetGameInstance`)))
  (bind _output_get_2 (set `self.GameInstanceRef` _ashcgame_instance))
  (`KismetArrayLibrary.Array_Add` (`/Game/Blueprints/HCGameInstance.SpawnedEnemies` _output_get_2) self)
  ;[1 0.2417 0.9092 0.396] Set gamemode ref
  (bind _ashero_cart_game_mode (cast `/Game/Blueprints/HeroCartGameMode` (`GameplayStatics.GetGameMode`)))
  (set `self.GameModeRef` _ashero_cart_game_mode))

(event `/Game/Blueprints/BlueprintExtras/I_Damageable.TakeDamage`
  (params (Damagers :type "Array of /Game/Blueprints/BlueprintExtras/S_Damage Structure (by ref)") (Instigator :type "Actor Object Reference") (AttackName :type String))
  (bind _addeddamage (`self.AddTotalDamage` Damagers))
  (bind _capsulecomponent (`self.CapsuleComponent`))
  ;[1 0 0.04473 0.813] Receive damage
  (if (`self.IsAlive`)
    (set `self.ReceivedHit` true)
    (bind _output_get (set `self.CurrentHealth` (- (`self.CurrentHealth`) _addeddamage)))
    (`/Game/Blueprints/HeroCartGameMode.DisplayDamage` (`self.GameModeRef`) false _addeddamage (`self.K2_GetActorLocation`) (1.0 1.0 1.0))
    (if (<= _output_get 0)
      (set `self.IsAlive` false)
      (set `self.CanMove` false)
      (`PrimitiveComponent.SetSimulatePhysics` (`self.Mesh`) true)
      (`PrimitiveComponent.SetCollisionEnabled` _capsulecomponent "NoCollision")
      (`PrimitiveComponent.SetSimulatePhysics` _capsulecomponent false)
      (`self.OnDeath`)
      (`/Game/Blueprints/HCGameInstance.Remove Enemy from List` (`self.GameInstanceRef`) self)
      (elif (== (`self.CurrentTarget`) null)
        ;[1 0.2929 0 0.583] Move to unknown attacker
        (if (`self.CanMove`)
          (`|AIMoveTo` self (0.0 0.0 0.0) Instigator (`self.MoveDistance`) true))))))

(event `OnDeath`
  (`self.SpawnLoot`))

(fn `AddTotalDamage`
  (params (DamageArray :type "Array of /Game/Blueprints/BlueprintExtras/S_Damage Structure"))
  (returns (AddedDamage :type Integer))
  (locals (TotalDamage :type Integer))
  (bind _totaldamage (`local.TotalDamage`))
  (for _array_element DamageArray
    (set `local.TotalDamage` (+ (`.DamageAmount_18_321AF0A24042A6CB9F954D8296FA0889` (break `/Game/Blueprints/BlueprintExtras/S_Damage` _array_element)) _totaldamage)))
  (return _totaldamage))

(fn `MultiplyDamageByLevel`
  (params (DamageArray :type "Array of /Game/Blueprints/BlueprintExtras/S_Damage Structure"))
  (returns (LeveledDamage :type "Array of /Game/Blueprints/BlueprintExtras/S_Damage Structure"))
  (locals (TempDamager :type "Array of /Game/Blueprints/BlueprintExtras/S_Damage Structure"))
  (bind _tempdamager (`local.TempDamager`))
  (for (_array_element _array_index) DamageArray
    (bind (_damagetype _damageamount) (break `/Game/Blueprints/BlueprintExtras/S_Damage` _array_element))
    (`KismetArrayLibrary.Array_Set` _tempdamager _array_index (make `/Game/Blueprints/BlueprintExtras/S_Damage` _damagetype (* _damageamount (`self.Level`))) true))
  (return _tempdamager))

(fn `SpawnLoot`
  (locals (TempRandomGold :type Integer))
  ;[1 1 1] Spawn random amount of gold; TODO: Add item drops
  (bind _output_get (set `local.TempRandomGold` (`KismetMathLibrary.RandomIntegerInRange` (`self.MinGoldDropped`) (`self.MaxGoldDropped`))))
  (if (> _output_get 0)
    (`|SpawnActorFromClass` "/Game/Blueprints/Pickables/PickableGold.PickableGold_C" (`KismetMathLibrary.Conv_VectorToTransform` (`self.K2_GetActorLocation`)) "AlwaysSpawn" "OverrideRootScale" null _output_get null)))

(fn `UserConstructionScript`)