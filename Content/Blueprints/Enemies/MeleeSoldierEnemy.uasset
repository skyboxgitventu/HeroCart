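; Melee soldier enemy that chases noises it hears and attacks at close range, built on a parent enemy class.
; PawnSensing hearing starts an AI move toward the noise instigator and sets it as the target.
; Tick turns smoothly toward the target, stops to flag cooldown-gated attacks in range, and destroys the actor after a delay once dead.
; HitReport sends level-scaled damage to hit actors through the I_Damageable interface.
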(event `self.ReceiveBeginPlay`
  (`parent.ReceiveBeginPlay`))

(event `HitReport`
  (params (ActorsHit :type "Array of Actor Object Reference"))
  ;[1 0 0.04473 0.813] Apply damage to targets hit
  (for _array_element ActorsHit
    (if (`KismetSystemLibrary.DoesImplementInterface` _array_element "/Game/Blueprints/BlueprintExtras/I_Damageable.I_Damageable_C")
      (message `/Game/Blueprints/BlueprintExtras/I_Damageable.TakeDamage` _array_element (`self.MultiplyDamageByLevel` (`self.BaseDamager`)) self "BaseEnemyLightAttack"))))

(event `self.ReceiveTick`
  (params (DeltaSeconds :type "Float (single-precision)"))
  (bind _currenttarget (`self.CurrentTarget`))
  (bind _capsulecomponent (`self.CapsuleComponent`))
  (bind _returnvalue (`KismetMathLibrary.Abs` (`KismetSystemLibrary.GetGameTimeInSeconds`)))
  (bind _returnvalue_2 (`self.K2_GetActorLocation` _currenttarget))
  (bind _returnvalue_3 (`SceneComponent.K2_GetComponentLocation` _capsulecomponent))
  (`parent.ReceiveTick` DeltaSeconds)
  ;[1 0 0.04473 0.813] Is alive?
  (if (`self.IsAlive`)
    ;[1 0.2417 0.9092 0.396] Has target
    (`/Engine/EditorBlueprintResources/StandardMacros.IsValid` _currenttarget
      (:`Is Valid`
        ;[1 0.2417 0.9092 0.396] If close enough to attack
        (if (<= (`KismetMathLibrary.Vector_Distance` _returnvalue_3 _returnvalue_2) (`self.AttackDistance`))
          ;[1 0 0.04473 0.813] Attack if cooldown ready
          (if (>= (- _returnvalue (`self.LastAttack`)) (`self.AttackCooldown`))
            (set `self.IsAttackingMelee` true)
            (set `self.LastAttack` _returnvalue)
            (`NavMovementComponent.StopActiveMovement` (`self.CharacterMovement`))))
        ;[1 0.2929 0 0.583] Otherwise look at target
        (`self.K2_SetActorRotation` (`KismetMathLibrary.MakeRotator` 0.0 0.0 (.yaw (`KismetMathLibrary.RLerp` (`SceneComponent.K2_GetComponentRotation` _capsulecomponent) (`KismetMathLibrary.FindLookAtRotation` _returnvalue_3 _returnvalue_2) 0.6 true))) true)))
    (else
      (`KismetSystemLibrary.Delay` 5.0)
      (`self.K2_DestroyActor`))))

(event `self.PawnSensing.OnHearNoise`
  (params (Instigator :type "Pawn Object Reference") (Location :type "Vector Structure (by ref)") (Volume :type "Float (single-precision)"))
  ;[1 0.2929 0 0.583] Move to player when sensing them
  (if (`self.IsAlive`)
    (if (`self.CanMove`)
      (if (not (`self.IsAttackingMelee`))
        (`|AIMoveTo` self (0.0 0.0 0.0) Instigator (`self.MoveDistance`) true
          (:`then`
            (set `self.CurrentTarget` Instigator)))))))

(fn `UserConstructionScript`)