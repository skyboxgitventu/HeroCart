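; Ranged caster enemy that moves toward noises it hears and attacks the instigator with level-scaled AOE magic orbs.
; Tick yaws it toward the target, flags an attack when in range and off cooldown, and destroys it after death.
; Orbs spawn motionless above the Head socket, aimed at the target, until an animation-driven event launches them.
; Death removes any unfired orb.
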(event `self.ReceiveBeginPlay`
  (`parent.ReceiveBeginPlay`))

(event `self.ReceiveTick`
  (params (DeltaSeconds :type "Float (single-precision)"))
  (bind _currenttarget (`self.CurrentTarget`))
  (bind _capsulecomponent (`self.CapsuleComponent`))
  (bind _returnvalue (`KismetMathLibrary.Abs` (`KismetSystemLibrary.GetGameTimeInSeconds`)))
  (bind _returnvalue_2 (`self.K2_GetActorLocation` _currenttarget))
  (bind _returnvalue_3 (`SceneComponent.K2_GetComponentLocation` _capsulecomponent))
  (`parent.ReceiveTick` DeltaSeconds)
  ;[1 0 0.04473 0.813] Is alive?
  (if (`self.IsAlive`)
    ;[1 0.2417 0.9092 0.396] Has target
    (`/Engine/EditorBlueprintResources/StandardMacros.IsValid` _currenttarget
      (:`Is Valid`
        ;[1 0.2417 0.9092 0.396] If close enough to attack
        (if (<= (`KismetMathLibrary.Vector_Distance` _returnvalue_3 _returnvalue_2) (`self.AttackDistance`))
          ;[1 0 0.04473 0.813] Attack if cooldown ready
          (if (>= (- _returnvalue (`self.LastAttack`)) (`self.AttackCooldown`))
            (set `self.IsAttacking` true)
            (set `self.LastAttack` _returnvalue)
            (`NavMovementComponent.StopActiveMovement` (`self.CharacterMovement`))
            ;[1 0.2929 0 0.583] Otherwise look at target
            (`self.K2_SetActorRotation` (`KismetMathLibrary.MakeRotator` 0.0 0.0 (.yaw (`KismetMathLibrary.RLerp` (`SceneComponent.K2_GetComponentRotation` _capsulecomponent) (`KismetMathLibrary.FindLookAtRotation` _returnvalue_3 _returnvalue_2) 0.6 true))) true :!label _label)
            (else
              (if (`self.CanRotate`) :!label _label_2
                (goto _label))))
          (else
            (goto _label_2)))))
    (else
      (`KismetSystemLibrary.Delay` 5.0)
      (`self.K2_DestroyActor`))))

(event `self.PawnSensing.OnHearNoise`
  (params (Instigator :type "Pawn Object Reference") (Location :type "Vector Structure (by ref)") (Volume :type "Float (single-precision)"))
  ;[1 0.2929 0 0.583] Move to player when sensing them
  (if (`self.IsAlive`)
    (if (`self.CanMove`)
      (if (not (`self.IsAttacking`))
        (`|AIMoveTo` self (0.0 0.0 0.0) Instigator (`self.MoveDistance`) true
          (:`then`
            (set `self.CurrentTarget` Instigator)))))))

(event `CreateProjectile`
  (bind _returnvalue (`SceneComponent.GetSocketLocation` (`self.Mesh`) "Head"))
  (bind _returnvalue_2 (`|SpawnActorFromClass` "/Game/Blueprints/Attacks/BaseProjectile.BaseProjectile_C" (`KismetMathLibrary.MakeTransform` (+ _returnvalue (0.0 0.0 100.0)) (`KismetMathLibrary.MakeRotator` 0.0 (.pitch (`KismetMathLibrary.FindLookAtRotation` _returnvalue (`self.K2_GetActorLocation` (`self.CurrentTarget`)))) (.yaw (`KismetMathLibrary.FindLookAtRotation` _returnvalue (`self.K2_GetActorLocation` (`self.CurrentTarget`)))))) "Undefined" "OverrideRootScale" null false 0.0 false false null (`self.MultiplyDamageByLevel` (`self.BaseDamage`)) true 200.0 "/Engine/BasicShapes/Sphere.Sphere" 1.0 7.0 "/Game/Blueprints/Heroes/BaseHeroClass.BaseHeroClass_C" self "Caster Magic Orb" 500.0 true 500.0 "NewEnumerator1" self))
  (set `self.CurrentProjectileRef` _returnvalue_2))

(event `ShootProjectile`
  (bind _currentprojectileref (`self.CurrentProjectileRef`))
  ;[1 0 0.04473 0.813] Enable projectile movement on anim event
  (`/Engine/EditorBlueprintResources/StandardMacros.IsValid` _currentprojectileref
    (:`Is Valid`
      (`ProjectileMovementComponent.SetVelocityInLocalSpace` (`/Game/Blueprints/Attacks/BaseProjectile.ProjectileMovement` _currentprojectileref) (1000.0 0.0 0.0))
      (set `self.CurrentProjectileRef` null))))

(event `self.OnDeath`
  (bind _currentprojectileref (`self.CurrentProjectileRef`))
  ;[1 0 0.04473 0.813] Remove projectile if spawned before shooting it
  (`/Engine/EditorBlueprintResources/StandardMacros.IsValid` _currentprojectileref
    (:`Is Valid`
      (`self.K2_DestroyActor` _currentprojectileref))))

(fn `UserConstructionScript`
  (`parent.UserConstructionScript`))