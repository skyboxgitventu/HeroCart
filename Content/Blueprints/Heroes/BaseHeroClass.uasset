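; Base hero actor providing health, damage, targeting and edit-mode placement controls for hero units.
; Health and outgoing damage scale with Level; incoming damage totals typed entries and clears IsAlive at zero, with helpers for cooldowns and ragdolling.
; FindValidTarget sphere-overlaps enemies, filters by a yaw vision cone, then picks a living one by distance or health according to TargetingMethod.
; In edit mode, mouse release selects the hero and dragging a selected hero rotates it.
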(event `self.ReceiveBeginPlay`
  (bind _plane (`self.Plane`))
  ;[0.2538 1 0 0.635] Set max health
  (bind _output_get (set `self.MaxHealth` (* (`self.MaxHealthPerLevel`) (`self.Level`))))
  (set `self.CurrentHealth` _output_get)
  ;[1 0.2417 0.9092 0.396] Set reference to game instance
  (bind _ashcgame_instance (cast `/Game/Blueprints/HCGameInstance` (`GameplayStatics.GetGameInstance`)))
  (set `self.GameInstance` _ashcgame_instance)
  ;[1 0.2417 0.9092 0.396] Set reference to player controller
  (bind _asdefault_player_controller (cast `/Game/Blueprints/DefaultPlayerController` (`GameplayStatics.GetPlayerController` 0)))
  (set `self.PlayerControllerRef` _asdefault_player_controller)
  ;[0 1 0.5318 0.417] Set FOV display on hero
  (`MeshComponent.SetScalarParameterValueOnMaterials` _plane "Angle" (`self.VisionAngle`))
  (`SceneComponent.SetVisibility` _plane false false))

(event `self.Mesh.OnClicked`
  (params (TouchedComponent :type "PrimitiveComponent Object Reference") (ButtonPressed :type "Key Structure"))
  ;[0 1 0.5318 0.417] OnClickEvent (start rotation if selected)
  (if (and (`self.GetIsInEditMode`) (== (`/Game/Blueprints/HCGameInstance.SelectedHero` (`self.GameInstance`)) self))
    (set `self.IsRotatingInEditor` true)
    (set `self.Original Rotation` 0.0)))

(event `self.Mesh.OnReleased`
  (params (TouchedComponent :type "PrimitiveComponent Object Reference") (ButtonReleased :type "Key Structure"))
  ;[0 1 0.5318 0.417] On release while in Edit Mode. TODO: Add click validator to prevent shenanigans
  (if (`self.GetIsInEditMode`)
    (`/Game/Blueprints/HCGameInstance.SelectHeroToEdit` (`self.GameInstance`) self)))

(event `self.ReceiveTick`
  (params (DeltaSeconds :type "Float (single-precision)"))
  (bind _playercontrollerref (`self.PlayerControllerRef`))
  (if (`self.IsRotatingInEditor`)
    (if (`/Game/Blueprints/DefaultPlayerController.LeftMouseDown` _playercontrollerref)
      ;[0 1 0.5318 0.417] Rotate actor in cart edit mode
      (bind _returnvalue (`WidgetLayoutLibrary.GetMousePositionOnViewport`))
      (bind _returnvalue_2 (- _returnvalue (`/Game/Blueprints/DefaultPlayerController.LastLeftMousePressLocation` _playercontrollerref)))
      (if (> (`KismetMathLibrary.VSize2D` _returnvalue_2) (`self.MinDistanceToRotate`))
        (bind (_x _y) (`KismetMathLibrary.BreakVector2D` _returnvalue_2))
        (`self.K2_SetActorRotation` (`KismetMathLibrary.MakeRotator` (.roll (`self.K2_GetActorRotation`)) (.pitch (`self.K2_GetActorRotation`)) (- (`KismetMathLibrary.DegAtan2` _y _x) (`self.Original Rotation`)))))
      (else
        ;[0 1 0.5318 0.417] Stop rotating on mouse up
        (set `self.IsRotatingInEditor` false)))))

(event `/Game/Blueprints/BlueprintExtras/I_Damageable.TakeDamage`
  (params (Damagers :type "Array of /Game/Blueprints/BlueprintExtras/S_Damage Structure (by ref)") (Instigator :type "Actor Object Reference") (AttackName :type String))
  (bind _totaldamage (`self.AddTotalDamage` Damagers))
  (bind _currenthealth (`self.CurrentHealth`))
  ;[1 0 0.04473 0.813] Hero taking damage
  (if (`self.IsAlive`)
    (bind _output_get (set `self.CurrentHealth` (- _currenthealth _totaldamage)))
    (`KismetSystemLibrary.PrintString` (`KismetStringLibrary.Concat_StrStr` (`KismetSystemLibrary.GetDisplayName` Instigator) " used " AttackName " on " (`self.HeroName`) " and inflicted " (`KismetStringLibrary.Conv_IntToString` _totaldamage) " points of damage - HEALTH: " (`KismetStringLibrary.Conv_IntToString` _currenthealth) " / " (`KismetStringLibrary.Conv_IntToString` (`self.MaxHealth`))))
    (if (<= _output_get 0)
      (set `self.IsAlive` false))))

(fn `AddTotalDamage`
  (params (Damagers :type "Array of /Game/Blueprints/BlueprintExtras/S_Damage Structure"))
  (returns (TotalDamage :type Integer))
  (locals (TempDamage :type Integer))
  (for _array_element Damagers
    (set `local.TempDamage` (+ (`.DamageAmount_18_321AF0A24042A6CB9F954D8296FA0889` (break `/Game/Blueprints/BlueprintExtras/S_Damage` _array_element)) (`local.TempDamage`))))
  (return (`local.TempDamage`)))

(fn `CalculateDamageByLevel`
  (params (BaseDamage :type "Array of /Game/Blueprints/BlueprintExtras/S_Damage Structure"))
  (returns (LeveledDamage :type "Array of /Game/Blueprints/BlueprintExtras/S_Damage Structure"))
  (locals (ReturnDamage :type "Array of /Game/Blueprints/BlueprintExtras/S_Damage Structure"))
  (bind _returndamage (`local.ReturnDamage`))
  ;[1 1 1] Base scale damage by Level. TODO: Add hero attributes and passive skill mods
  (for (_array_element _array_index) BaseDamage
    (bind (_damagetype _damageamount) (break `/Game/Blueprints/BlueprintExtras/S_Damage` _array_element))
    (`KismetArrayLibrary.Array_Set` _returndamage _array_index (make `/Game/Blueprints/BlueprintExtras/S_Damage` _damagetype (* _damageamount (`self.Level`))) true))
  (return _returndamage))

(fn `CheckCoolDownTimer`
  (params (LastAttackTime :type "Float (double-precision)") (AttackCooldown :type "Float (double-precision)"))
  (returns (CooldownReady :type Boolean))
  (bind _returnvalue (- (`KismetMathLibrary.Conv_FloatToDouble` (`KismetSystemLibrary.GetGameTimeInSeconds`)) LastAttackTime))
  ;[1 1 1] Compare cooldown with last skill use timestamp
  (set `self.CooldownRatio` (`KismetMathLibrary.SafeDivide` _returnvalue AttackCooldown))
  (return (>= _returnvalue AttackCooldown)))

(fn `FindValidTarget`
  (returns (BestTarget :type "Actor Object Reference"))
  (locals (TempCompareValue :type "Float (double-precision)" :default 9999999.0) (TempTargets :type "Array of Actor Object Reference") (ReturnTarget :type "Actor Object Reference"))
  (bind _temptargets (`local.TempTargets`))
  ;[1 1 1] Find enemies in detect radius
  (bind (_outactors _returnvalue) (`KismetSystemLibrary.SphereOverlapActors` (`self.K2_GetActorLocation` self) (`self.SightRadius`) (`|MakeArray` "ObjectTypeQuery7" :!type "EObjectTypeQuery Enum") "/Game/Blueprints/Enemies/BaseEnemyClass.BaseEnemyClass_C" (`|MakeArray` self :!type "Actor Object Reference")))
  ;[1 1 1] Filter by sight cone
  (if _returnvalue
    (for _array_element _outactors
      (if (not (> (`KismetMathLibrary.Abs` (.yaw (`KismetMathLibrary.FindRelativeLookAtRotation` (`self.GetTransform` self) (`self.K2_GetActorLocation` _array_element)))) (`self.VisionAngle`)))
        (`KismetArrayLibrary.Array_Add` _temptargets _array_element)))
    ;[1 1 1] If there is at least one enemy
    (if (> (`KismetArrayLibrary.Array_Length` _temptargets) 0)
      ;[1 1 1] Expand to include more modes and friendly targeting
      (switch `/Game/Blueprints/BlueprintExtras/E_TargetingMethod` (`self.TargetingMethod`)
        (:`NewEnumerator0`
          ;[1 1 1] Sort by shortest distance
          (set `local.TempCompareValue` 9999999.0)
          (for _array_element_2 _temptargets
            (bind _asbase_enemy_class (cast `/Game/Blueprints/Enemies/BaseEnemyClass` _array_element_2))
            (bind _returnvalue_2 (`KismetMathLibrary.Vector_Distance` (`self.K2_GetActorLocation` _array_element_2) (`self.K2_GetActorLocation` self)))
            (if (and (< _returnvalue_2 (`local.TempCompareValue`)) (`/Game/Blueprints/Enemies/BaseEnemyClass.IsAlive` _asbase_enemy_class))
              (set `local.ReturnTarget` _array_element_2)
              (set `local.TempCompareValue` _returnvalue_2))))
        (:`NewEnumerator1`
          ;[1 1 1] Sort by longest distance
          (set `local.TempCompareValue` 0.0)
          (for _array_element_3 _temptargets
            (bind _asbase_enemy_class_2 (cast `/Game/Blueprints/Enemies/BaseEnemyClass` _array_element_3))
            (bind _returnvalue_3 (`KismetMathLibrary.Vector_Distance` (`self.K2_GetActorLocation` _array_element_3) (`self.K2_GetActorLocation` self)))
            (if (and (> _returnvalue_3 (`local.TempCompareValue`)) (`/Game/Blueprints/Enemies/BaseEnemyClass.IsAlive` _asbase_enemy_class_2))
              (set `local.ReturnTarget` _array_element_3)
              (set `local.TempCompareValue` _returnvalue_3))))
        (:`NewEnumerator2`
          ;[1 1 1] Sort by most health
          (set `local.TempCompareValue` 0.0)
          (for _array_element_4 _temptargets
            (bind _asbase_enemy_class_3 (cast `/Game/Blueprints/Enemies/BaseEnemyClass` _array_element_4))
            (bind _currenthealth (`/Game/Blueprints/Enemies/BaseEnemyClass.CurrentHealth` _asbase_enemy_class_3))
            (if (and (> _currenthealth (`local.TempCompareValue`)) (`/Game/Blueprints/Enemies/BaseEnemyClass.IsAlive` _asbase_enemy_class_3))
              (set `local.ReturnTarget` _array_element_4)
              (set `local.TempCompareValue` (`KismetMathLibrary.Conv_IntToDouble` _currenthealth)))))
        (:`NewEnumerator3`
          ;[1 1 1] Sort by less health
          (set `local.TempCompareValue` 9999999.0)
          (for _array_element_5 _temptargets
            (bind _asbase_enemy_class_4 (cast `/Game/Blueprints/Enemies/BaseEnemyClass` _array_element_5))
            (bind _currenthealth_2 (`/Game/Blueprints/Enemies/BaseEnemyClass.CurrentHealth` _asbase_enemy_class_4))
            (if (and (< _currenthealth_2 (`local.TempCompareValue`)) (`/Game/Blueprints/Enemies/BaseEnemyClass.IsAlive` _asbase_enemy_class_4))
              (set `local.ReturnTarget` _array_element_5)
              (set `local.TempCompareValue` (`KismetMathLibrary.Conv_IntToDouble` _currenthealth_2))))))
      (return (`local.ReturnTarget`))
      (else
        (return null)))
    (else
      (return null))))

(fn `GetIsInEditMode`
  (returns (IsInEditMode :type Boolean))
  ;[1 1 1] Check if game instance is in any of the edit modes
  (return (`|EnumEquality` (`/Game/Blueprints/HCGameInstance.CurrentMode` (`self.GameInstance`)) "NewEnumerator1")))

(fn `TurnIntoRagdoll`
  (bind _capsulecomponent (`self.CapsuleComponent`))
  (`PrimitiveComponent.SetSimulatePhysics` (`self.Mesh`) true)
  (`PrimitiveComponent.SetCollisionEnabled` _capsulecomponent "NoCollision")
  (`PrimitiveComponent.SetSimulatePhysics` _capsulecomponent false))

(fn `UserConstructionScript`)