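; Warrior hero Blueprint that automatically attacks enemies with a melee swing.
; Outside edit mode, Tick checks alive state, attack state and cooldown, then finds a valid target, stamps the attack time and sets the attack flag.
; HitReport sends damage to hit actors through the I_Damageable interface, passing each actor's hit index times a per-enemy increase as the per-level damage bonus.
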(event `self.ReceiveTick`
  (params (DeltaSeconds :type "Float (single-precision)"))
  ;[1 0 0.04473 0.813] Attack cycle (check cooldown, look for enemies, attack)
  (`parent.ReceiveTick` DeltaSeconds)
  (if (not (`self.GetIsInEditMode`))
    (bind _cooldownready (`self.CheckCoolDownTimer` (`self.LastAttack1`) (`self.MainAttackCooldown`)))
    (if (and (not (`self.IsAttacking`)) (`self.IsAlive`) _cooldownready)
      (set `self.AttackTarget` null)
      (bind _besttarget (`self.FindValidTarget`))
      (`/Engine/EditorBlueprintResources/StandardMacros.IsValid` _besttarget
        (:`Is Valid`
          (set `self.LastAttack1` (`KismetMathLibrary.Conv_FloatToDouble` (`KismetSystemLibrary.GetGameTimeInSeconds`)))
          (set `self.ShouldAttack` true)
          (set `self.AttackTarget` _besttarget))))))

(event `HitReport`
  (params (ActorsHit :type "Array of Actor Object Reference"))
  (if (> (`KismetArrayLibrary.Array_Length` ActorsHit) 0)
    (for (_array_element _array_index) ActorsHit
      (if (`KismetSystemLibrary.DoesImplementInterface` _array_element "/Game/Blueprints/BlueprintExtras/I_Damageable.I_Damageable_C")
        (message `/Game/Blueprints/BlueprintExtras/I_Damageable.TakeDamage` _array_element (`self.CalculateDamageByLevel` (`self.BaseDamage`) (* _array_index (`self.DamageIncreasePerEnemy`))) self "Melee Hero Swing")))))

(fn `UserConstructionScript`)