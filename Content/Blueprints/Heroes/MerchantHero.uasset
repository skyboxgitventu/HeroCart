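; MerchantHero is a hero Blueprint that runs a cooldown-gated combat check on top of its parent class logic.
; Each Tick outside edit mode, while the hero is alive and the main attack cooldown check passes, it searches for a valid target.
; A found target stamps the last attack time and sets the in-combat flag, otherwise the flag clears.
; This graph makes no attack or damage call itself.
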(event `self.ReceiveTick`
  (params (DeltaSeconds :type "Float (single-precision)"))
  ;[1 0 0.04473 0.813] Attack cycle (check cooldown, look for enemies, attack)
  (`parent.ReceiveTick` DeltaSeconds)
  (if (not (`self.GetIsInEditMode`))
    (bind _cooldownready (`self.CheckCoolDownTimer` (`self.LastAttack1`) (`self.MainAttackCooldown`)))
    (if (and (`self.IsAlive`) _cooldownready)
      (bind _besttarget (`self.FindValidTarget`))
      (`/Engine/EditorBlueprintResources/StandardMacros.IsValid` _besttarget
        (:`Is Valid`
          (set `self.LastAttack1` (`KismetMathLibrary.Conv_FloatToDouble` (`KismetSystemLibrary.GetGameTimeInSeconds`)))
          (set `self.IsInCombat` true))
        (:`Is Not Valid`
          (set `self.IsInCombat` false))))))

(fn `UserConstructionScript`
  (`parent.UserConstructionScript`))