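; World map Blueprint that procedurally builds a tiered list of towns running from a start point to a last point.
; GenerateWorldMap fills TownList with a random number of placeholder-named towns per middle stage, then calls SetRoadConnections.
; SetRoadConnections calculates roads per town and a remainder for each adjacent tier pair, but its connection-writing loop is unwired, so no roads are assigned.
; The event graph and construction script are empty.
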(fn `GenerateWorldMap`
  (locals (TempRandom :type Integer) (TempTownArray :type "Array of /Game/Blueprints/BlueprintExtras/S_MapTownInfo Structure"))
  (bind _numberofstages (`self.NumberOfStages`))
  (bind _townlist (`self.TownList`))
  (bind _temptownarray (`local.TempTownArray`))
  ;[1 1 1] Add First entry to world map
  (`KismetArrayLibrary.Array_Add` _townlist (make `/Game/Blueprints/BlueprintExtras/S_TierTowns` (`|MakeArray` (make `/Game/Blueprints/BlueprintExtras/S_MapTownInfo` "START POINT"))))
  ;[1 1 1] Make mid towns
  (for _index (range _numberofstages)
    (`KismetArrayLibrary.Array_Clear` (`local.TempTownArray`))
    (bind _output_get (set `local.TempRandom` (`KismetMathLibrary.RandomIntegerInRange` 1 (`self.MaxTownsPerStage`))))
    (for _ (range _output_get)
      (`KismetArrayLibrary.Array_Add` _temptownarray (make `/Game/Blueprints/BlueprintExtras/S_MapTownInfo` "RANDOM TOWN NAME" (+ _index 1))))
    (`KismetArrayLibrary.Array_Add` (`self.TownList`) (make `/Game/Blueprints/BlueprintExtras/S_TierTowns` _temptownarray)))
  ;[1 1 1] Add Last entry to world map
  (`KismetArrayLibrary.Array_Add` _townlist (make `/Game/Blueprints/BlueprintExtras/S_TierTowns` (`|MakeArray` (make `/Game/Blueprints/BlueprintExtras/S_MapTownInfo` "LAST POINT" _numberofstages))))
  (`self.SetRoadConnections`))

(fn `SetRoadConnections`
  (locals (TempNumberOfRoadsToAssign :type Integer) (TempIndex :type Integer) (TempConnection :type Integer) (TempRoadsPerNode :type Integer) (Remainder :type Integer))
  (bind _townlist (`self.TownList`))
  (for _index (range (+ (- (`KismetArrayLibrary.Array_Length` _townlist) 2) 1))
    (set `local.TempConnection` 0)
    (set `local.TempIndex` 0)
    (bind _returnvalue (`KismetArrayLibrary.Array_Length` (`.TownsInTier_5_82A9006444477C15629FA7A9192E2A89` (break `/Game/Blueprints/BlueprintExtras/S_TierTowns` (`|GetArrayItem` _townlist _index)))))
    (bind _output_get (set `local.TempNumberOfRoadsToAssign` (`KismetMathLibrary.Max` _returnvalue (`KismetArrayLibrary.Array_Length` (`.TownsInTier_5_82A9006444477C15629FA7A9192E2A89` (break `/Game/Blueprints/BlueprintExtras/S_TierTowns` (`|GetArrayItem` _townlist (+ _index 1))))))))
    (bind _output_get_2 (set `local.TempRoadsPerNode` (/ _output_get _returnvalue)))
    (set `local.Remainder` (- _output_get (* _returnvalue _output_get_2)))))

(fn `UserConstructionScript`)