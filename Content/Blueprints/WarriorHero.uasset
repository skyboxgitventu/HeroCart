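; Melee warrior hero that automatically attacks valid targets and damages what its swing hits.
; Outside edit mode and when not already attacking, Tick checks the attack cooldown, finds a target, timestamps the attack and sets ShouldAttack and AttackTarget.
; Damage is applied separately in HitReport, which sends level-scaled damage to every reported actor implementing I_Damageable, not just the chosen target.
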(event `self.ReceiveTick`
  (params (DeltaSeconds :type "Float (single-precision)"))
  ;[1 0 0.04473 0.813] Attack cycle (check cooldown, look for enemies, attack)
  (if (`self.IsInEditMode`)
    _
    (elif (not (`self.IsAttacking`))
      (bind _cooldownready (`self.CheckCoolDownTimer` (`self.LastAttack1`) (`self.Attack1Cooldown`)))
      (if _cooldownready
        (set `self.AttackTarget` null)
        (bind _besttarget (`self.FindValidTarget`))
        (`/Engine/EditorBlueprintResources/StandardMacros.IsValid` _besttarget
          (:`Is Valid`
            (set `self.LastAttack1` (`KismetMathLibrary.Conv_FloatToDouble` (`KismetSystemLibrary.GetGameTimeInSeconds`)))
            (set `self.ShouldAttack` true)
            (set `self.AttackTarget` _besttarget)))))))

(event `HitReport`
  (params (ActorsHit :type "Array of Actor Object Reference"))
  (for _array_element ActorsHit
    (if (`KismetSystemLibrary.DoesImplementInterface` _array_element "/Game/Blueprints/BlueprintExtras/I_Damageable.I_Damageable_C")
      (message `/Game/Blueprints/BlueprintExtras/I_Damageable.TakeDamage` _array_element (`self.CalculateDamageByLevel` (`self.Damage`)) self "Melee Hero Swing"))))

(fn `UserConstructionScript`)