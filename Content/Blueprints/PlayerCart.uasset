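; Player-controlled cart pawn that drives forward under physics and rams enemies.
; Axis input sets a desired heading, and RotateTowardsTarget yaws the mesh toward it in fixed steps along the shortest wrapped angle.
; While moving, Tick applies clamped forward force, emits AI noise, and on a cooldown sphere-checks ahead to damage BaseEnemy pawns through I_Damageable.
; Received damage is only printed, and the debug direction arrows are disconnected.
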(event `InputAxis|YAXIS`
  (params (AxisValue :type "Float (single-precision)"))
  (bind _playermesh (`self.PlayerMesh`))
  (bind _cartdeadzone (`self.CartDeadZone`))
  (bind _returnvalue (`SceneComponent.GetForwardVector` _playermesh))
  ;[0 1 0.5318 0.417] Rotation input
  (if (or (> (`KismetMathLibrary.Abs` AxisValue) _cartdeadzone) (> (`KismetMathLibrary.Abs` (stale `InputAxis|XAXIS` AxisValue)) _cartdeadzone)) :!label _label
    (bind _output_get (set `self.DesiredDirection` (`KismetMathLibrary.MakeVector` (stale `InputAxis|XAXIS` AxisValue) AxisValue)))
    (else
      (set `self.DesiredDirection` _returnvalue)))
  (`self.Rotate Towards Target` (`KismetMathLibrary.Vector_HeadingAngle` _output_get) (`KismetMathLibrary.Vector_HeadingAngle` (`KismetMathLibrary.Normal` _returnvalue)) (`self.CartRotationSpeed`) _playermesh))

(event `InputAxis|XAXIS`
  (params (AxisValue :type "Float (single-precision)"))
  ;[0 1 0.5318 0.417] Rotation input
  (goto _label))

(event `self.ReceiveTick`
  (params (DeltaSeconds :type "Float (single-precision)"))
  (bind _returnvalue (`KismetSystemLibrary.GetGameTimeInSeconds`))
  (bind _playermesh (`self.PlayerMesh`))
  (bind _returnvalue_2 (`SceneComponent.GetForwardVector` (`self.PlayerMesh`)))
  (bind _returnvalue_3 (`SceneComponent.K2_GetComponentLocation` (`self.PlayerMesh`)))
  ;[1 0.2929 0 0.583] Cart movement
  (if (`self.ShouldBeMoving`)
    (`PawnNoiseEmitterComponent.MakeNoise` (`self.PawnNoiseEmitter`) self 1.0 _returnvalue_3)
    (`PrimitiveComponent.AddForce` _playermesh (* (`self.CartAcceleration`) (`KismetMathLibrary.Normal` _returnvalue_2)) "None" true)
    (bind _returnvalue_4 (`PrimitiveComponent.GetPhysicsLinearVelocity` _playermesh "None"))
    (`PrimitiveComponent.SetPhysicsLinearVelocity` _playermesh (`KismetMathLibrary.ClampVectorSize` _returnvalue_4 0.0 (`self.CartMaxSpeed`)) false "None")
    (if (>= (- (`KismetMathLibrary.Abs` _returnvalue) (`self.LastCartAttackTime`)) (`self.CartAttackCooldown`))
      (set `self.LastCartAttackTime` _returnvalue)
      (bind (_outactors _returnvalue_5) (`KismetSystemLibrary.SphereOverlapActors` (+ _returnvalue_3 (* _returnvalue_2 100.0)) 100.0 (`|MakeArray` "ObjectTypeQuery3" :!type "EObjectTypeQuery Enum") "/Game/Blueprints/BaseEnemy.BaseEnemy_C"))
      (if _returnvalue_5
        (for _array_element _outactors
          (if (`KismetSystemLibrary.DoesImplementInterface` _array_element "/Game/Blueprints/BlueprintExtras/I_Damageable.I_Damageable_C")
            (message `/Game/Blueprints/BlueprintExtras/I_Damageable.TakeDamage` _array_element (`self.CartBaseDamage`) self "CartCollision")))))))

(event `/Game/Blueprints/BlueprintExtras/I_Damageable.TakeDamage`
  (params (Damagers :type "Array of /Game/Blueprints/BlueprintExtras/S_Damage Structure (by ref)") (Instigator :type "Actor Object Reference") (AttackName :type String))
  (for _array_element Damagers
    (`KismetSystemLibrary.PrintString` (`KismetStringLibrary.Concat_StrStr` (`KismetSystemLibrary.GetDisplayName` Instigator) " used " AttackName " on " (`KismetSystemLibrary.GetDisplayName` self) " and inflicted " (`KismetStringLibrary.Conv_IntToString` (`.DamageAmount_18_321AF0A24042A6CB9F954D8296FA0889` (break `/Game/Blueprints/BlueprintExtras/S_Damage` _array_element))) " points of damage"))))

(fn `Rotate Towards Target`
  (params (DesiredDirection :type "Float (double-precision)") (CurrentDirection :type "Float (double-precision)") (RotationSpeed :type "Float (double-precision)") (MeshToRotate :type "StaticMeshComponent Object Reference"))
  (locals (Diff :type "Float (double-precision)" :default -0.1) (AngleThreshold :type "Float (double-precision)" :default 0.001) (RotationDelta :type "Rotator Structure" :default (struct)))
  (bind _returnvalue (`KismetMathLibrary.GetPI`))
  (bind _diff (`local.Diff`))
  (bind _returnvalue_2 (* _returnvalue 2.0))
  (bind _returnvalue_3 (- (mod (+ (- CurrentDirection DesiredDirection) _returnvalue) _returnvalue_2) _returnvalue))
  (if (<= _returnvalue_3 (* _returnvalue -1.0))
    (set `local.Diff` (+ _returnvalue_3 _returnvalue_2))
    (else
      (set `local.Diff` _returnvalue_3)))
  (if (>= (`KismetMathLibrary.Abs` _diff) (`local.AngleThreshold`))
    (if (< _diff 0.0)
      (set `local.RotationDelta` (`KismetMathLibrary.MakeRotator` 0.0 0.0 RotationSpeed))
      (else
        (bind _output_get (set `local.RotationDelta` (`KismetMathLibrary.MakeRotator` 0.0 0.0 (* RotationSpeed -1.0))))))
    (`SceneComponent.K2_AddWorldRotation` MeshToRotate _output_get false false)
    (return)))

(fn `UserConstructionScript`)