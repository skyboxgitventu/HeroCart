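; Base hero class that supplies health setup and combat helper functions, setting max and current health from level on BeginPlay.
; FindValidTarget sphere-overlaps enemies within sight radius, filters them by a yaw vision cone, then picks a living one by targeting method: closest, furthest, most health or least health.
; Other helpers test attack cooldown against game time and multiply each typed damage entry by hero level.
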(event `self.ReceiveBeginPlay`
  ;[0.2538 1 0 0.635] Set max health
  (bind _output_get (set `self.MaxHealth` (* (`self.MaxHealthPerLevel`) (`self.Level`))))
  (set `self.CurrentHealth` _output_get))

(fn `CalculateDamageByLevel`
  (params (BaseDamage :type "Array of /Game/Blueprints/BlueprintExtras/S_Damage Structure"))
  (returns (LeveledDamage :type "Array of /Game/Blueprints/BlueprintExtras/S_Damage Structure"))
  (locals (ReturnDamage :type "Array of /Game/Blueprints/BlueprintExtras/S_Damage Structure"))
  (bind _returndamage (`local.ReturnDamage`))
  (for (_array_element _array_index) BaseDamage
    (bind (_damagetype _damageamount) (break `/Game/Blueprints/BlueprintExtras/S_Damage` _array_element))
    (`KismetArrayLibrary.Array_Set` _returndamage _array_index (make `/Game/Blueprints/BlueprintExtras/S_Damage` _damagetype (* _damageamount (`self.Level`))) true))
  (return _returndamage))

(fn `CheckCoolDownTimer`
  (params (LastAttackTime :type "Float (double-precision)") (AttackCooldown :type "Float (double-precision)"))
  (returns (CooldownReady :type Boolean))
  (return (>= (- (`KismetMathLibrary.Conv_FloatToDouble` (`KismetSystemLibrary.GetGameTimeInSeconds`)) LastAttackTime) AttackCooldown)))

(fn `FindValidTarget`
  (returns (BestTarget :type "Actor Object Reference"))
  (locals (TempCompareValue :type "Float (double-precision)" :default 9999999.0) (TempTargets :type "Array of Actor Object Reference") (ReturnTarget :type "Actor Object Reference"))
  (bind _temptargets (`local.TempTargets`))
  ;[1 1 1] Find enemies in detect radius
  (bind (_outactors _returnvalue) (`KismetSystemLibrary.SphereOverlapActors` (`self.K2_GetActorLocation` self) (`self.SightRadius`) (`|MakeArray` "ObjectTypeQuery7" :!type "EObjectTypeQuery Enum") "/Game/Blueprints/BaseEnemyClass.BaseEnemyClass_C" (`|MakeArray` self :!type "Actor Object Reference")))
  ;[1 1 1] Filter by sight cone
  (if _returnvalue
    (for _array_element _outactors
      (if (not (> (`KismetMathLibrary.Abs` (.yaw (`KismetMathLibrary.FindRelativeLookAtRotation` (`self.GetTransform` self) (`self.K2_GetActorLocation` _array_element)))) (`self.VisionAngle`)))
        (`KismetArrayLibrary.Array_Add` _temptargets _array_element)))
    ;[1 1 1] If there is at least one enemy
    (if (> (`KismetArrayLibrary.Array_Length` _temptargets) 0)
      ;[1 1 1] Expand to include more modes and friendly targeting
      (switch `/Game/Blueprints/BlueprintExtras/E_TargetingMethod` (`self.TargetingMethod`)
        (:`NewEnumerator0`
          ;[1 1 1] Sort by shortest distance
          (set `local.TempCompareValue` 9999999.0)
          (for _array_element_2 _temptargets
            (bind _asbase_enemy_class (cast `/Game/Blueprints/BaseEnemyClass` _array_element_2))
            (bind _returnvalue_2 (`KismetMathLibrary.Vector_Distance` (`self.K2_GetActorLocation` _array_element_2) (`self.K2_GetActorLocation` self)))
            (if (and (< _returnvalue_2 (`local.TempCompareValue`)) (`/Game/Blueprints/BaseEnemyClass.IsAlive` _asbase_enemy_class))
              (set `local.ReturnTarget` _array_element_2)
              (set `local.TempCompareValue` _returnvalue_2))))
        (:`NewEnumerator1`
          ;[1 1 1] Sort by longest distance
          (set `local.TempCompareValue` 0.0)
          (for _array_element_3 _temptargets
            (bind _asbase_enemy_class_2 (cast `/Game/Blueprints/BaseEnemyClass` _array_element_3))
            (bind _returnvalue_3 (`KismetMathLibrary.Vector_Distance` (`self.K2_GetActorLocation` _array_element_3) (`self.K2_GetActorLocation` self)))
            (if (and (> _returnvalue_3 (`local.TempCompareValue`)) (`/Game/Blueprints/BaseEnemyClass.IsAlive` _asbase_enemy_class_2))
              (set `local.ReturnTarget` _array_element_3)
              (set `local.TempCompareValue` _returnvalue_3))))
        (:`NewEnumerator2`
          ;[1 1 1] Sort by most health
          (set `local.TempCompareValue` 0.0)
          (for _array_element_4 _temptargets
            (bind _asbase_enemy_class_3 (cast `/Game/Blueprints/BaseEnemyClass` _array_element_4))
            (bind _currenthealth (`/Game/Blueprints/BaseEnemyClass.CurrentHealth` _asbase_enemy_class_3))
            (if (and (> _currenthealth (`local.TempCompareValue`)) (`/Game/Blueprints/BaseEnemyClass.IsAlive` _asbase_enemy_class_3))
              (set `local.ReturnTarget` _array_element_4)
              (set `local.TempCompareValue` (`KismetMathLibrary.Conv_IntToDouble` _currenthealth)))))
        (:`NewEnumerator3`
          ;[1 1 1] Sort by less health
          (set `local.TempCompareValue` 9999999.0)
          (for _array_element_5 _temptargets
            (bind _asbase_enemy_class_4 (cast `/Game/Blueprints/BaseEnemyClass` _array_element_5))
            (bind _currenthealth_2 (`/Game/Blueprints/BaseEnemyClass.CurrentHealth` _asbase_enemy_class_4))
            (if (and (< _currenthealth_2 (`local.TempCompareValue`)) (`/Game/Blueprints/BaseEnemyClass.IsAlive` _asbase_enemy_class_4))
              (set `local.ReturnTarget` _array_element_5)
              (set `local.TempCompareValue` (`KismetMathLibrary.Conv_IntToDouble` _currenthealth_2))))))
      (return (`local.ReturnTarget`))
      (else
        (return null)))
    (else
      (return null))))

(fn `UserConstructionScript`)