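; CartSlot is a clickable hero slot on the cart that selects or assigns heroes while the game instance is in one specific mode.
; Press records the slot on the player controller, so release acts only when both hit the same slot, then clears that target.
; With a hero selected, release assigns it here through the game instance.
; With none selected, or the same one, it selects the slot's occupant for editing.
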(event `self.ReceiveBeginPlay`
  (bind _ashcgame_instance (cast `/Game/Blueprints/HCGameInstance` (`GameplayStatics.GetGameInstance`)))
  (set `self.GameInstance` _ashcgame_instance))

(event `self.MiniatureBase.OnReleased`
  (params (TouchedComponent :type "PrimitiveComponent Object Reference") (ButtonReleased :type "Key Structure"))
  (bind _gameinstance (`self.GameInstance`))
  (bind _assignedhero (`self.AssignedHero`))
  (bind _selectedhero (`/Game/Blueprints/HCGameInstance.SelectedHero` _gameinstance))
  (bind _returnvalue (== _selectedhero null))
  ;[1 1 1] If click and release were done on same target
  (if (`|EnumEquality` (`/Game/Blueprints/HCGameInstance.CurrentMode` (`self.GameInstance`)) "NewEnumerator1")
    (bind _asdefault_player_controller (cast `/Game/Blueprints/DefaultPlayerController` (`GameplayStatics.GetPlayerController` 0)))
    (if (== self (`/Game/Blueprints/DefaultPlayerController.TargetClickForValidation` _asdefault_player_controller))
      ;[1 1 1] Is this slot empty
      (if (== _assignedhero null)
        (if _returnvalue
          (set `/Game/Blueprints/DefaultPlayerController.TargetClickForValidation` null _asdefault_player_controller) ; Clicked on empty slot
          (else
            ;[1 1 1] Assign selected hero to clicked slot
            (`/Game/Blueprints/HCGameInstance.AssignSelectedHeroToSlot` _gameinstance self :!label _label)
            (set `/Game/Blueprints/DefaultPlayerController.TargetClickForValidation` null _asdefault_player_controller)))
        (else
          (if _returnvalue
            _
            (elif (== _selectedhero _assignedhero)
              _
              (else
                (goto _label))))
          ;[1 1 1] Select hero if none selected
          (`/Game/Blueprints/HCGameInstance.SelectHeroToEdit` _gameinstance _assignedhero)
          (set `/Game/Blueprints/DefaultPlayerController.TargetClickForValidation` null _asdefault_player_controller)))
      (else
        (set `/Game/Blueprints/DefaultPlayerController.TargetClickForValidation` null _asdefault_player_controller)))))

(event `self.MiniatureBase.OnClicked`
  (params (TouchedComponent :type "PrimitiveComponent Object Reference") (ButtonPressed :type "Key Structure"))
  ;[1 1 1] Set initial click target for validation
  (if (`|EnumEquality` (`/Game/Blueprints/HCGameInstance.CurrentMode` (`self.GameInstance`)) "NewEnumerator1")
    (bind _asdefault_player_controller (cast `/Game/Blueprints/DefaultPlayerController` (`GameplayStatics.GetPlayerController` 0)))
    (set `/Game/Blueprints/DefaultPlayerController.TargetClickForValidation` self _asdefault_player_controller)))

(fn `UserConstructionScript`)