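; Player cart pawn for Hero Cart that drives itself during Travel mode, rams enemies and carries hero slots.
; Axis input steers the mesh by shortest-angle yaw steps, while Tick applies speed-clamped physics force and emits AI noise.
; A front box periodically deals level-scaled damage through I_Damageable.
; Incoming damage reduces level-based health, with death triggering a fade and game over; helpers handle travel, HUD, gold and level restart.
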(event `self.ReceiveBeginPlay`
  ;[0.2538 1 0 0.635] TEMP Set Initial health
  (bind _output_get (set `self.MaxHealth` (* (`self.Level`) (`self.MaxHealthPerLevel`))))
  (set `self.CurrentHealth` _output_get)
  (`self.UpdateCartSlots`)
  (bind _ashcgame_instance (cast `/Game/Blueprints/HCGameInstance` (`GameplayStatics.GetGameInstance`)))
  (bind _output_get_2 (set `self.GameRef` _ashcgame_instance))
  (bind _ashero_cart_game_mode (cast `/Game/Blueprints/HeroCartGameMode` (`GameplayStatics.GetGameMode`)))
  (set `self.GameModeRef` _ashero_cart_game_mode)
  (switch `/Game/Blueprints/BlueprintExtras/E_GameMode` (`/Game/Blueprints/HCGameInstance.CurrentMode` _output_get_2)))

(event `InputAxis|YAXIS`
  (params (AxisValue :type "Float (single-precision)"))
  (bind _playermesh (`self.PlayerMesh`))
  (bind _cartdeadzone (`self.CartDeadZone`))
  (bind _returnvalue (`SceneComponent.GetForwardVector` _playermesh))
  ;[0 1 0.5318 0.417] Rotation input
  (if (and (or (> (`KismetMathLibrary.Abs` AxisValue) _cartdeadzone) (> (`KismetMathLibrary.Abs` (stale `InputAxis|XAXIS` AxisValue)) _cartdeadzone)) (`self.IsCartAlive`)) :!label _label
    (bind _output_get (set `self.DesiredDirection` (`KismetMathLibrary.MakeVector` (stale `InputAxis|XAXIS` AxisValue) AxisValue)))
    (else
      (set `self.DesiredDirection` _returnvalue)))
  (`self.Rotate Towards Target` (`KismetMathLibrary.Vector_HeadingAngle` _output_get) (`KismetMathLibrary.Vector_HeadingAngle` (`KismetMathLibrary.Normal` _returnvalue)) (`self.CartRotationSpeed`) _playermesh))

(event `InputAxis|XAXIS`
  (params (AxisValue :type "Float (single-precision)"))
  ;[0 1 0.5318 0.417] Rotation input
  (goto _label))

(event `self.ReceiveTick`
  (params (DeltaSeconds :type "Float (single-precision)"))
  (bind _returnvalue (`KismetSystemLibrary.GetGameTimeInSeconds`))
  (bind _playermesh (`self.PlayerMesh`))
  (bind _attackbox (`self.AttackBox`))
  ;[1 0.2929 0 0.583] Cart movement
  (if (and (`|EnumEquality` (`/Game/Blueprints/HCGameInstance.CurrentMode` (`self.GameRef`)) "NewEnumerator2") (`self.ShouldBeMoving`) (`self.IsCartAlive`))
    (`PawnNoiseEmitterComponent.MakeNoise` (`self.PawnNoiseEmitter`) self 1.0 (`SceneComponent.K2_GetComponentLocation` (`self.PlayerMesh`)))
    (`PrimitiveComponent.AddForce` _playermesh (* (`self.CartAcceleration`) (`KismetMathLibrary.Normal` (`SceneComponent.GetForwardVector` (`self.PlayerMesh`)))) "None" true)
    (bind _returnvalue_2 (`PrimitiveComponent.GetPhysicsLinearVelocity` _playermesh "None"))
    (`PrimitiveComponent.SetPhysicsLinearVelocity` _playermesh (`KismetMathLibrary.ClampVectorSize` _returnvalue_2 0.0 (`self.CartMaxSpeed`)) false "None")
    ;[1 0 0.04473 0.813] Cart front melee attack
    (if (>= (- (`KismetMathLibrary.Abs` _returnvalue) (`self.LastCartAttackTime`)) (`self.CartAttackCooldown`))
      (set `self.LastCartAttackTime` _returnvalue)
      (bind (_outactors _returnvalue_3) (`KismetSystemLibrary.ComponentOverlapActors` _attackbox (`SceneComponent.K2_GetComponentToWorld` _attackbox) (`|MakeArray` "ObjectTypeQuery7" :!type "EObjectTypeQuery Enum")))
      (if _returnvalue_3
        (for _array_element _outactors
          (if (`KismetSystemLibrary.DoesImplementInterface` _array_element "/Game/Blueprints/BlueprintExtras/I_Damageable.I_Damageable_C")
            (message `/Game/Blueprints/BlueprintExtras/I_Damageable.TakeDamage` _array_element (`self.ApplyLevelToDamager`) self "CartCollision")))))))

(event `/Game/Blueprints/BlueprintExtras/I_Damageable.TakeDamage`
  (params (Damagers :type "Array of /Game/Blueprints/BlueprintExtras/S_Damage Structure (by ref)") (Instigator :type "Actor Object Reference") (AttackName :type String))
  (bind _totaldamage (`self.AddTotalDamage` Damagers))
  (bind _currenthealth (`self.CurrentHealth`))
  ;[1 0 0.04473 0.813] Taking damage
  (if (`self.IsCartAlive`)
    (set `self.CurrentHealth` (- _currenthealth _totaldamage))
    (`/Game/Blueprints/HeroCartGameMode.DisplayDamage` (`self.GameModeRef`) false _totaldamage (`self.K2_GetActorLocation`) (1.0 0.0 0.0))
    ;[1 0 0.04473 0.813] Cart is dead
    (if (<= _currenthealth 0)
      (`self.CartDead`)
      (`KismetSystemLibrary.PrintString` "GAME OVER" true true (struct :`R` 1.0 :`G` 0.033849 :`A` 1.0))
      (`KismetSystemLibrary.Delay` 3.0)
      (`/Game/Blueprints/HCGameInstance.GameOver` (`self.GameRef`)))))

(fn `AddTotalDamage`
  (params (Damager :type "Array of /Game/Blueprints/BlueprintExtras/S_Damage Structure"))
  (returns (TotalDamage :type Integer))
  (locals (TempDamage :type Integer))
  (for _array_element Damager
    (set `local.TempDamage` (+ (`.DamageAmount_18_321AF0A24042A6CB9F954D8296FA0889` (break `/Game/Blueprints/BlueprintExtras/S_Damage` _array_element)) (`local.TempDamage`))))
  (return (`local.TempDamage`)))

(fn `ApplyLevelToDamager`
  (returns (ModifiedDamage :type "Array of /Game/Blueprints/BlueprintExtras/S_Damage Structure"))
  (locals (ReturnDamage :type "Array of /Game/Blueprints/BlueprintExtras/S_Damage Structure"))
  (bind _returndamage (`local.ReturnDamage`))
  (for (_array_element _array_index) (`self.CartBaseDamage`)
    (bind (_damagetype _damageamount) (break `/Game/Blueprints/BlueprintExtras/S_Damage` _array_element))
    (`KismetArrayLibrary.Array_Set` _returndamage _array_index (make `/Game/Blueprints/BlueprintExtras/S_Damage` _damagetype (* _damageamount (`self.Level`))) true))
  (return _returndamage))

(fn `CartDead`
  ;[1 1 1] Set cart alive param
  (if (`self.IsCartAlive`)
    (set `self.IsCartAlive` false)
    (`LevelSequencePlayer.CreateLevelSequencePlayer` "/Game/Sequences/FadeToBlack.FadeToBlack" (make `MovieSceneSequencePlaybackSettings` true))))

(fn `GainXP`)

(fn `PickupGold`
  (params (Amount :type Integer))
  (bind _gameref (`self.GameRef`))
  (set `/Game/Blueprints/HCGameInstance.RoadGold` (+ Amount (`/Game/Blueprints/HCGameInstance.RoadGold` _gameref)) _gameref))

(fn `Restart Level`
  (set `/Game/Blueprints/HCGameInstance.CurrentMode` "NewEnumerator1" (`self.GameRef`))
  (bind _returnvalue (`GameplayStatics.GetCurrentLevelName` true))
  (`GameplayStatics.OpenLevel` (`KismetStringLibrary.Conv_StringToName` _returnvalue)))

(fn `Rotate Towards Target`
  (params (DesiredDirection :type "Float (double-precision)") (CurrentDirection :type "Float (double-precision)") (RotationSpeed :type "Float (double-precision)") (MeshToRotate :type "StaticMeshComponent Object Reference"))
  (locals (Diff :type "Float (double-precision)" :default -0.1) (AngleThreshold :type "Float (double-precision)" :default 0.001) (RotationDelta :type "Rotator Structure" :default (struct)))
  (bind _returnvalue (`KismetMathLibrary.GetPI`))
  (bind _diff (`local.Diff`))
  (bind _returnvalue_2 (* _returnvalue 2.0))
  (bind _returnvalue_3 (- (mod (+ (- CurrentDirection DesiredDirection) _returnvalue) _returnvalue_2) _returnvalue))
  (if (<= _returnvalue_3 (* _returnvalue -1.0))
    (set `local.Diff` (+ _returnvalue_3 _returnvalue_2))
    (else
      (set `local.Diff` _returnvalue_3)))
  (if (>= (`KismetMathLibrary.Abs` _diff) (`local.AngleThreshold`))
    (if (< _diff 0.0)
      (set `local.RotationDelta` (`KismetMathLibrary.MakeRotator` 0.0 0.0 RotationSpeed))
      (else
        (bind _output_get (set `local.RotationDelta` (`KismetMathLibrary.MakeRotator` 0.0 0.0 (* RotationSpeed -1.0))))))
    (`SceneComponent.K2_AddWorldRotation` MeshToRotate _output_get false false)
    (return)))

(fn `StartTravel`
  (`SceneComponent.SetVisibility` (`self.CartSlot1`) false false)
  (`SceneComponent.SetVisibility` (`self.CartSlot0`) false false)
  (`AudioComponent.Play` (`self.Audio`) 0.0)
  (set `self.ShouldBeMoving` true))

(fn `StopTravel`
  (`AudioComponent.Stop` (`self.Audio`))
  (set `self.ShouldBeMoving` false))

(fn `UpdateCartSlots`
  (bind _cartslots (`self.CartSlots`))
  (`KismetArrayLibrary.Array_Add` _cartslots (`self.CartSlot0`))
  (`KismetArrayLibrary.Array_Add` _cartslots (`self.CartSlot1`))
  (`self.UpdateHUD`))

(fn `UpdateHUD`
  (bind _ashero_cart_game_mode (cast `/Game/Blueprints/HeroCartGameMode` (`GameplayStatics.GetGameMode`)))
  (`/Game/Blueprints/UI/MainHUD.UpdateHeroIcons` (`/Game/Blueprints/HeroCartGameMode.MainHUD` _ashero_cart_game_mode) self))

(fn `UserConstructionScript`)