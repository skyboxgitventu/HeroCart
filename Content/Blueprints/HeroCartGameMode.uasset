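; HeroCartGameMode is the game mode for a cart game, running a wall of death that chases the player's cart during travel.
; BeginPlay creates the main HUD, caches the player cart and game instance, then starts initial cart configuration or travel based on the current mode.
; Tick advances the wall's X in a post-process Material Parameter Collection, which doubles as gameplay state: a cart behind it dies, triggering game over after a delay.
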(event `self.ReceiveTick`
  (params (DeltaSeconds :type "Float (single-precision)"))
  (bind _playercartref (`self.PlayerCartRef`))
  ;[1 0 0.04473 0.813] Move the wall of death forward while in travel mode
  (if (`|EnumEquality` (`/Game/Blueprints/HCGameInstance.CurrentMode` (`self.GameInstanceRef`)) "NewEnumerator2")
    (bind _returnvalue (`KismetMaterialLibrary.GetScalarParameterValue` "/Game/VFX/PostProcess/PostProcessGlobalParameters.PostProcessGlobalParameters" "WallOfDeathX"))
    (bind _returnvalue_2 (+ _returnvalue (* (`self.WallOfDeathSpeed`) DeltaSeconds)))
    (`KismetMaterialLibrary.SetScalarParameterValue` "/Game/VFX/PostProcess/PostProcessGlobalParameters.PostProcessGlobalParameters" "WallOfDeathX" _returnvalue_2)
    ;[1 0 0.04473 0.813] Death by wall of death
    (if (`/Game/Blueprints/HeroCartPlayer/PlayerCart.IsCartAlive` _playercartref)
      (if (< (.x (`self.K2_GetActorLocation` _playercartref)) _returnvalue_2)
        (`/Game/Blueprints/HeroCartPlayer/PlayerCart.CartDead` _playercartref)
        (`KismetSystemLibrary.Delay` 3.0)
        (`/Game/Blueprints/HCGameInstance.GameOver` (`self.GameInstanceRef`))))))

(event `self.ReceiveBeginPlay`
  (bind _returnvalue (`GameplayStatics.GetGameInstance`))
  ;[0 1 0.5318 0.417] Create Main HUD
  (bind _returnvalue_2 (`|CreateWidget` "/Game/Blueprints/UI/MainHUD.MainHUD_C"))
  (`UserWidget.AddToViewport` _returnvalue_2 0)
  (set `self.MainHUD` _returnvalue_2)
  ;[1 0.2417 0.9092 0.396] Set player ref
  (bind _asplayer_cart (cast `/Game/Blueprints/HeroCartPlayer/PlayerCart` (`GameplayStatics.GetPlayerPawn` 0)))
  (set `self.PlayerCartRef` _asplayer_cart)
  ;[1 0.2417 0.9092 0.396] Check game mode on start
  (`/Engine/EditorBlueprintResources/StandardMacros.IsValid` _returnvalue
    (:`Is Valid`
      (bind _ashcgame_instance (cast `/Game/Blueprints/HCGameInstance` _returnvalue))
      (bind _output_get (set `self.GameInstanceRef` _ashcgame_instance))
      (switch `/Game/Blueprints/BlueprintExtras/E_GameMode` (`/Game/Blueprints/HCGameInstance.CurrentMode` _output_get)
        (:`NewEnumerator1`
          (`/Game/Blueprints/HCGameInstance.StartInitialCartConfigMode` _ashcgame_instance))
        (:`NewEnumerator2`
          (`/Game/Blueprints/HCGameInstance.GoTravel` _ashcgame_instance))))))

(fn `UserConstructionScript`)