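; Cart configuration diorama actor that holds four cart slots and can populate them with randomly generated heroes.
; The construction script gathers the slot child actor components into the CartSlots array.
; FillSlotsWithRandomHeroes asks the supplied GameInstance for a level 1, tier 1 hero at each slot's transform, then cross-links hero and CartSlot references.
; The event graph has no active logic.
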(fn `FillSlotsWithRandomHeroes`
  (params (GameInstance :type "/Game/Blueprints/HCGameInstance Object Reference"))
  ;[1 1 1] Create one level 1 hero per slot, and assign slot->hero and hero->slot references
  (for _array_element (`self.CartSlots`)
    (bind _newhero (`/Game/Blueprints/HCGameInstance.MakeNewRandomHero` GameInstance 1 1 (`SceneComponent.K2_GetComponentToWorld` _array_element)))
    (bind _ascart_slot (cast `/Game/Blueprints/HeroCartPlayer/CartSlot` (`ChildActorComponent.ChildActor` _array_element)))
    (set `/Game/Blueprints/HeroCartPlayer/CartSlot.AssignedHero` _newhero _ascart_slot)
    (set `/Game/Blueprints/Heroes/BaseHeroClass.AttachedToSlot` _ascart_slot _newhero)))

(fn `UserConstructionScript`
  (bind _cartslots (`self.CartSlots`))
  (`KismetArrayLibrary.Array_Add` _cartslots (`self.CartSlot0`))
  (`KismetArrayLibrary.Array_Add` _cartslots (`self.CartSlot1`))
  (`KismetArrayLibrary.Array_Add` _cartslots (`self.CartSlot2`))
  (`KismetArrayLibrary.Array_Add` _cartslots (`self.CartSlot3`)))