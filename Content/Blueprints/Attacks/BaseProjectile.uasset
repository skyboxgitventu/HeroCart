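; Base configurable attack projectile that explodes on impact or lifetime expiry, with optional bouncing, homing, gravity and area damage.
; Construction script applies spawn parameters to movement, mesh and radial force, and sets collision channels by friend-or-foe side.
; Bouncy shots explode only on hitting the target class.
; Explode disables the mesh, spawns Niagara VFX, sends I_Damageable damage via sphere overlap or supplied actor, optionally fires an impulse, then delays destruction.
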(event `self.ReceiveTick`
  (params (DeltaSeconds :type "Float (single-precision)"))
  ;[1 1 1] Check lifespan
  (if (`self.IsActive`)
    (if (>= (- (`KismetMathLibrary.Conv_FloatToDouble` (`KismetSystemLibrary.GetGameTimeInSeconds`)) (`self.SpawnTime`)) (`self.Lifetime`))
      (`self.Explode` null))))

(event `self.ReceiveBeginPlay`
  (bind _trailvfx (`self.TrailVFX`))
  ;[1 1 1] Set spawn timer
  (set `self.SpawnTime` (`KismetMathLibrary.Conv_FloatToDouble` (`KismetSystemLibrary.GetGameTimeInSeconds`)))
  (`PrimitiveComponent.IgnoreActorWhenMoving` (`self.ProjectileMesh`) (`self.ProjectileOwner`) true)
  (if (`KismetSystemLibrary.IsValid` _trailvfx)
    (bind _returnvalue (`AddComponent|NODE_AddNiagaraComponent-1`))
    (`NiagaraComponent.SetAsset` _returnvalue _trailvfx true)))

(event `self.ProjectileMesh.OnComponentHit`
  (params (HitComponent :type "PrimitiveComponent Object Reference") (OtherActor :type "Actor Object Reference") (OtherComp :type "PrimitiveComponent Object Reference") (NormalImpulse :type "Vector Structure") (Hit :type "HitResult Structure (by ref)"))
  ;[1 1 1] Collision
  (if (`self.IsActive`)
    (if (`self.Bouncy`)
      (if (`KismetMathLibrary.ClassIsChildOf` (`GameplayStatics.GetObjectClass` OtherActor) (`self.TargetClass`))
        (`self.Explode` null))
      (else
        (`self.Explode` null)))))

(event `Explode`
  (params (ValidActorHit :type "Actor Object Reference"))
  (bind _projectilemesh (`self.ProjectileMesh`))
  (bind _damage (`self.Damage`))
  (bind _projectileowner (`self.ProjectileOwner`))
  (bind _attackname (`self.AttackName`))
  (bind _explosionvfx (`self.ExplosionVFX`))
  ;[1 1 1] Disable object
  (set `self.IsActive` false)
  (`SceneComponent.SetVisibility` _projectilemesh false true)
  (`PrimitiveComponent.SetSimulatePhysics` _projectilemesh false)
  (`PrimitiveComponent.SetCollisionEnabled` _projectilemesh "NoCollision")
  ;[1 1 1] Draw explosion VFX
  (`/Engine/EditorBlueprintResources/StandardMacros.IsValid` _explosionvfx
    (:`Is Valid`
      (bind _returnvalue (`AddComponent|NODE_AddNiagaraComponent-2`))
      (`NiagaraComponent.SetAsset` _returnvalue _explosionvfx true))
    (:`Is Not Valid`
      _))
  ;[1 1 1] Is AOE attack
  (if (`self.IsAOE`)
    (bind (_outactors _returnvalue_2) (`KismetSystemLibrary.SphereOverlapActors` (`SceneComponent.K2_GetComponentLocation` _projectilemesh) (`self.AOERadius`) (`self.CollisionTypesToCheck`) null (`|MakeArray` (`self.ProjectileOwner`))))
    (if _returnvalue_2
      (for _array_element _outactors
        (if (`KismetSystemLibrary.DoesImplementInterface` _array_element "/Game/Blueprints/BlueprintExtras/I_Damageable.I_Damageable_C")
          (message `/Game/Blueprints/BlueprintExtras/I_Damageable.TakeDamage` _array_element _damage _projectileowner _attackname)))
      ;[1 1 1] Apply impulse
      (if (`self.ApplyImpulse`) :!label _label
        (`RadialForceComponent.FireImpulse` (`self.RadialForce`))))
    (else
      ;[1 1 1] Not AOE
      (`/Engine/EditorBlueprintResources/StandardMacros.IsValid` ValidActorHit
        (:`Is Valid`
          (if (`KismetSystemLibrary.DoesImplementInterface` ValidActorHit "/Game/Blueprints/BlueprintExtras/I_Damageable.I_Damageable_C")
            (message `/Game/Blueprints/BlueprintExtras/I_Damageable.TakeDamage` ValidActorHit _damage _projectileowner _attackname)
            (goto _label)
            (else
              _)))
        (:`Is Not Valid`
          _))))
  ;[1 1 1] Destroy the actor after delay for VFX
  (`KismetSystemLibrary.Delay` 3.0)
  (`self.K2_DestroyActor`))

(fn `UserConstructionScript`
  (bind _projectilemovement (`self.ProjectileMovement`))
  (bind _homing (`self.Homing`))
  (bind _homingtarget (`self.HomingTarget`))
  (bind _projectilemesh (`self.ProjectileMesh`))
  ;[1 1 1] Set initial parameters from spawn
  (set `ProjectileMovementComponent.ProjectileGravityScale` (`KismetMathLibrary.Conv_BoolToDouble` (`self.GravityEnabled`)) _projectilemovement)
  (bind _output_get (set `ProjectileMovementComponent.InitialSpeed` (`self.Speed`) _projectilemovement))
  (set `ProjectileMovementComponent.MaxSpeed` (* (`KismetMathLibrary.Conv_FloatToDouble` _output_get) 2.0) _projectilemovement)
  (set `ProjectileMovementComponent.bShouldBounce` (`self.Bouncy`) _projectilemovement)
  (set `ProjectileMovementComponent.bIsHomingProjectile` _homing _projectilemovement)
  (if (and _homing (`KismetSystemLibrary.IsValid` _homingtarget))
    (set `ProjectileMovementComponent.HomingTargetComponent` (`Actor.RootComponent` _homingtarget) _projectilemovement)
    (set `self.HomingSpeed` (`self.HomingSpeed`)))
  (`StaticMeshComponent.SetStaticMesh` _projectilemesh (`self.Mesh`))
  (`SceneComponent.SetRelativeScale3D` _projectilemesh (`KismetMathLibrary.Conv_DoubleToVector` (`self.Scale`)))
  (set `RadialForceComponent.ImpulseStrength` (`self.ImpulseStrength`) (`self.RadialForce`))
  (`PrimitiveComponent.SetMaterial` _projectilemesh 0 (`self.MeshMaterial`))
  (switch `/Game/Blueprints/BlueprintExtras/E_FriendOrFoe` (`self.FriendOrFoe`)
    (:`NewEnumerator0`
      (`PrimitiveComponent.SetCollisionResponseToChannel` _projectilemesh "ECC_GameTraceChannel2" "ECR_Ignore")
      (`PrimitiveComponent.SetCollisionResponseToChannel` _projectilemesh "ECC_GameTraceChannel1" "ECR_Block")
      (`PrimitiveComponent.SetCollisionObjectType` _projectilemesh "ECC_GameTraceChannel2")
      (set `self.CollisionTypesToCheck` (`|MakeArray` "ObjectTypeQuery7" :!type "EObjectTypeQuery Enum")))
    (:`NewEnumerator1`
      (`PrimitiveComponent.SetCollisionResponseToChannel` _projectilemesh "ECC_GameTraceChannel1" "ECR_Ignore")
      (`PrimitiveComponent.SetCollisionResponseToChannel` _projectilemesh "ECC_GameTraceChannel2" "ECR_Block")
      (`PrimitiveComponent.SetCollisionObjectType` _projectilemesh "ECC_GameTraceChannel1")
      (set `self.CollisionTypesToCheck` (`|MakeArray` "ObjectTypeQuery8" :!type "EObjectTypeQuery Enum")))))