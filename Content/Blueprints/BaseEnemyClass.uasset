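; Base enemy Blueprint that handles level-scaled health, incoming damage and death.
; BeginPlay sets health from Level; TakeDamage subtracts the summed damage array and prints a combat message.
; At zero health the mesh switches to physics and capsule collision is disabled; otherwise, a targetless, mobile enemy moves toward its attacker.
; A helper, unused in this graph, multiplies damage entries by Level.
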(event `self.ReceiveBeginPlay`
  ;[0.2538 1 0 0.635] SetMaxHealth
  (bind _output_get (set `self.MaxHealth` (* (`self.MaxHealthPerLevel`) (`self.Level`))))
  (set `self.CurrentHealth` _output_get))

(event `self.ReceiveTick`
  (params (DeltaSeconds :type "Float (single-precision)")))

(event `/Game/Blueprints/BlueprintExtras/I_Damageable.TakeDamage`
  (params (Damagers :type "Array of /Game/Blueprints/BlueprintExtras/S_Damage Structure (by ref)") (Instigator :type "Actor Object Reference") (AttackName :type String))
  (bind _addeddamage (`self.AddTotalDamage` Damagers))
  (bind _capsulecomponent (`self.CapsuleComponent`))
  ;[1 0 0.04473 0.813] Receive damage
  (if (`self.IsAlive`)
    (set `self.ReceivedHit` true)
    (bind _output_get (set `self.CurrentHealth` (- (`self.CurrentHealth`) _addeddamage)))
    (`KismetSystemLibrary.PrintString` (`KismetStringLibrary.Concat_StrStr` (`KismetSystemLibrary.GetDisplayName` Instigator) " used " AttackName " on " (`KismetSystemLibrary.GetDisplayName` self) " and inflicted " (`KismetStringLibrary.Conv_IntToString` _addeddamage) " points of damage. HEALTH: " (`KismetStringLibrary.Conv_IntToString` (`self.CurrentHealth`)) " / " (`KismetStringLibrary.Conv_IntToString` (`self.MaxHealth`))))
    (if (<= _output_get 0)
      (set `self.IsAlive` false)
      (set `self.CanMove` false)
      (`PrimitiveComponent.SetSimulatePhysics` (`self.Mesh`) true)
      (`PrimitiveComponent.SetCollisionEnabled` _capsulecomponent "NoCollision")
      (`PrimitiveComponent.SetSimulatePhysics` _capsulecomponent false)
      (elif (== (`self.CurrentTarget`) null)
        ;[1 0.2929 0 0.583] Move to unknown attacker
        (if (`self.CanMove`)
          (`|AIMoveTo` self (0.0 0.0 0.0) Instigator (`self.MoveDistance`) true))))))

(fn `AddTotalDamage`
  (params (DamageArray :type "Array of /Game/Blueprints/BlueprintExtras/S_Damage Structure"))
  (returns (AddedDamage :type Integer))
  (locals (TotalDamage :type Integer))
  (bind _totaldamage (`local.TotalDamage`))
  (for _array_element DamageArray
    (set `local.TotalDamage` (+ (`.DamageAmount_18_321AF0A24042A6CB9F954D8296FA0889` (break `/Game/Blueprints/BlueprintExtras/S_Damage` _array_element)) _totaldamage)))
  (return _totaldamage))

(fn `MultiplyDamageByLevel`
  (params (DamageArray :type "Array of /Game/Blueprints/BlueprintExtras/S_Damage Structure"))
  (returns (LeveledDamage :type "Array of /Game/Blueprints/BlueprintExtras/S_Damage Structure"))
  (locals (TempDamager :type "Array of /Game/Blueprints/BlueprintExtras/S_Damage Structure"))
  (bind _tempdamager (`local.TempDamager`))
  (for (_array_element _array_index) DamageArray
    (bind (_damagetype _damageamount) (break `/Game/Blueprints/BlueprintExtras/S_Damage` _array_element))
    (`KismetArrayLibrary.Array_Set` _tempdamager _array_index (make `/Game/Blueprints/BlueprintExtras/S_Damage` _damagetype (* _damageamount (`self.Level`))) true))
  (return _tempdamager))

(fn `UserConstructionScript`)