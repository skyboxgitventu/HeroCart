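; WitchHero is a hero that lobs area-of-effect fireballs at enemies.
; Tick checks the attack cooldown when idle, finds a valid target, stores it and flags ShouldAttack.
; ShootProjectile, a separate event, spawns a BaseProjectile from the right-hand socket with level-scaled damage and impulse.
; The gravity-affected shot launches at 45 degrees yawed toward the target, with speed derived from the square root of distance times gravity and a fixed multiplier.
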(event `self.ReceiveTick`
  (params (DeltaSeconds :type "Float (single-precision)"))
  ;[1 0 0.04473 0.813] Attack cycle (check cooldown, look for enemies, attack)
  (if (not (`self.IsAttacking`))
    (bind _cooldownready (`self.CheckCoolDownTimer` (`self.LastAttack1`) (`self.Attack1Cooldown`)))
    (if _cooldownready
      (set `self.AttackTarget` null)
      (bind _besttarget (`self.FindValidTarget`))
      (`/Engine/EditorBlueprintResources/StandardMacros.IsValid` _besttarget
        (:`Is Valid`
          (set `self.LastAttack1` (`KismetMathLibrary.Conv_FloatToDouble` (`KismetSystemLibrary.GetGameTimeInSeconds`)))
          (set `self.ShouldAttack` true)
          (set `self.AttackTarget` _besttarget))))))

(event `ShootProjectile`
  (bind _returnvalue (`self.K2_GetActorLocation` (`self.AttackTarget`)))
  (bind _returnvalue_2 (`SceneComponent.GetSocketLocation` (`self.Mesh`) "RightHand"))
  (`|SpawnActorFromClass` "/Game/Blueprints/Attacks/BaseProjectile.BaseProjectile_C" (`KismetMathLibrary.MakeTransform` (+ _returnvalue_2 (* (`KismetMathLibrary.Normal` (- _returnvalue _returnvalue_2)) (`self.ProjectileOffset`))) (`KismetMathLibrary.MakeRotator` 0.0 45.0 (.yaw (`KismetMathLibrary.FindLookAtRotation` _returnvalue_2 _returnvalue)))) "Undefined" "OverrideRootScale" null true (* (`KismetMathLibrary.Sqrt` (* (`KismetMathLibrary.Vector_Distance` _returnvalue_2 _returnvalue) 9.8)) 9.0) false false null (`self.CalculateDamageByLevel` (`self.Damage`)) true 300.0 "/Engine/BasicShapes/Sphere.Sphere" 0.5 10.0 "/Game/Blueprints/BaseEnemyClass.BaseEnemyClass_C" self "Witch Fireball" 500.0 true 500.0 self))

(fn `UserConstructionScript`)