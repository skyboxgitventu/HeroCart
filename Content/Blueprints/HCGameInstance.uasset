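; Game instance for the hero cart game, driving the loop of cart setup, road travel, arrival tally, town and game-over level reload.
; It spawns random heroes into diorama and town slots, handling selection, moves and swaps between slots.
; Travel builds levels from start, random middle and end tiles, switches cameras and enables a material-parameter wall of death.
; Arrival clears enemies and opens the tally screen, with helpers scoring living and dead heroes.
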(fn `Activate Town Camera`
  (`PlayerController.SetViewTargetWithBlend` (`GameplayStatics.GetPlayerController` 0) (`ChildActorComponent.ChildActor` (`/Game/Blueprints/Environment/Towns/TownBaseClass.TownCamera` (`self.CurrentTown`))) 0.0 "VTBlend_Linear" 0.0 false))

(fn `ArrivedToTown`
  ;[1 1 1] Fade to black
  (bind (_outactor _returnvalue) (`LevelSequencePlayer.CreateLevelSequencePlayer` "/Game/Sequences/FadeToBlack.FadeToBlack" (make `MovieSceneSequencePlaybackSettings` true (make `MovieSceneSequenceLoopCount` 0) 1.0 0.0 false false false false false false false true)))
  (add `MovieSceneSequencePlayer.OnFinished` _returnvalue (`|CreateDelegate` :!event `ClearLevel`))
  ;[1 1 1] Remove enemies and stop cart
  (`self.ClearEnemies`)
  (`/Game/Blueprints/HeroCartPlayer/PlayerCart.StopTravel` (`self.PlayerCartRef`))
  ;[1 1 1] Create Tally screen and add to viewport
  (bind _returnvalue_2 (`|CreateWidget` "/Game/Blueprints/UI/EndOfRoadScreen.EndOfRoadScreen_C"))
  (`UserWidget.AddToViewport` _returnvalue_2 0)
  ;[1 1 1] Reset wall of death
  (`KismetMaterialLibrary.SetScalarParameterValue` "/Game/VFX/PostProcess/PostProcessGlobalParameters.PostProcessGlobalParameters" "WallOfDeathX" -5500.0)
  (`KismetMaterialLibrary.SetScalarParameterValue` "/Game/VFX/PostProcess/PostProcessGlobalParameters.PostProcessGlobalParameters" "WallOfDeathAlpha")
  (set `self.IsMainHUDVisible` false))

(fn `AssignSelectedHeroToSlot`
  (params (TargetSlot :type "/Game/Blueprints/HeroCartPlayer/CartSlot Object Reference"))
  (bind _selectedhero (`self.SelectedHero`))
  (bind _assignedhero (`/Game/Blueprints/HeroCartPlayer/CartSlot.AssignedHero` TargetSlot))
  ;[1 1 1] Both slot and hero are valid
  (if (and (`KismetSystemLibrary.IsValid` TargetSlot) (`KismetSystemLibrary.IsValid` _selectedhero))
    ;[1 1 1] Target slot is empty?
    (if (== _assignedhero null)
      (`self.SetHeroSlot` _selectedhero TargetSlot true)
      (else
        ;[1 1 1] Replace old hero before moving new one
        (`self.SetHeroSlot` _assignedhero (`/Game/Blueprints/Heroes/BaseHeroClass.AttachedToSlot` _selectedhero))
        (`self.SetHeroSlot` _selectedhero TargetSlot)))))

(fn `ClearEnemies`
  (bind _spawnedenemies (`self.SpawnedEnemies`))
  (for _array_element _spawnedenemies
    (`/Engine/EditorBlueprintResources/StandardMacros.IsValid` _array_element
      (:`Is Valid`
        (`Actor.K2_DestroyActor` _array_element))))
  (`KismetArrayLibrary.Array_Clear` _spawnedenemies))

(fn `ClearHeroSelection`
  (bind _selectedhero (`self.SelectedHero`))
  ;[1 1 1] Remove selection and disable FOV display
  (`/Engine/EditorBlueprintResources/StandardMacros.IsValid` _selectedhero
    (:`Is Valid`
      (`SceneComponent.SetVisibility` (`/Game/Blueprints/Heroes/BaseHeroClass.Plane` _selectedhero) false true)
      (set `self.SelectedHero` null))))

(fn `ClearLevel`
  (bind _leveltiles (`self.LevelTiles`))
  (for _array_element _leveltiles
    (`Actor.K2_DestroyActor` _array_element))
  (`KismetArrayLibrary.Array_Clear` _leveltiles)
  (set `self.CurrentMode` "NewEnumerator4")
  (`self.SetupTown`))

(fn `DisplayTownWelcomeText`
  (bind _returnvalue (`|CreateWidget` "/Game/Blueprints/UI/WelcomeToLocationWidget.WelcomeToLocationWidget_C"))
  (set `/Game/Blueprints/UI/WelcomeToLocationWidget.TownName` (`KismetStringLibrary.ToUpper` (`/Game/Blueprints/Environment/Towns/TownBaseClass.TownName` (`self.CurrentTown`))) _returnvalue)
  (`UserWidget.AddToViewport` _returnvalue 0))

(fn `EnterTown`
  ;[1 1 1] Fade in
  (`LevelSequencePlayer.CreateLevelSequencePlayer` "/Game/Sequences/FadeFromBlack.FadeFromBlack" (make `MovieSceneSequencePlaybackSettings` true (make `MovieSceneSequenceLoopCount` 0) 1.0 0.0 false false false false false false false true))
  ;[1 1 1] Set camera, display welcome text, re enable cart slots
  (`self.Activate Town Camera`)
  (`self.DisplayTownWelcomeText`)
  (set `self.IsMainHUDVisible` true)
  (`/Game/Blueprints/HeroCartPlayer/PlayerCart.SetCartSlotsVisible` (`self.PlayerCartRef`) true)
  (`/Game/Blueprints/Environment/Towns/TownBaseClass.SetLocationColliders` (`self.CurrentTown`) true))

(fn `GameOver`
  (set `self.CurrentMode` "NewEnumerator1")
  (bind _returnvalue (`GameplayStatics.GetCurrentLevelName` true))
  (`GameplayStatics.OpenLevel` (`KismetStringLibrary.Conv_StringToName` _returnvalue)))

(fn `GetAliveRoadBonus`
  (returns (Gold :type Integer) (XP :type Integer))
  (locals (TempXP :type Integer) (TempGold :type Integer))
  ;[1 1 1] Check if each hero assigned to a slot is alive
  (for _array_element (`/Game/Blueprints/HeroCartPlayer/PlayerCart.CartSlots` (`self.PlayerCartRef`))
    (bind _ascart_slot (cast `/Game/Blueprints/HeroCartPlayer/CartSlot` (`ChildActorComponent.ChildActor` _array_element)))
    (bind _assignedhero (`/Game/Blueprints/HeroCartPlayer/CartSlot.AssignedHero` _ascart_slot))
    ;[1 1 1] Add bonus if alive
    (if (`KismetSystemLibrary.IsValid` _assignedhero)
      (if (`/Game/Blueprints/Heroes/BaseHeroClass.IsAlive` _assignedhero)
        (bind _level (`/Game/Blueprints/Heroes/BaseHeroClass.Level` _assignedhero))
        (set `local.TempGold` (+ (* _level (`/Game/Blueprints/Heroes/BaseHeroClass.GoldBonusAlive` _assignedhero)) (`local.TempGold`)))
        (set `local.TempXP` (+ (* _level (`/Game/Blueprints/Heroes/BaseHeroClass.XPBonusAlive` _assignedhero)) (`local.TempXP`))))))
  (return (`local.TempGold`) (`local.TempXP`)))

(fn `GetDeadRoadPenalty`
  (returns (Gold :type Integer) (XP :type Integer))
  (locals (TempGold :type Integer) (TempXP :type Integer))
  ;[1 1 1] Check if each hero assigned to a slot is alive
  (for _array_element (`/Game/Blueprints/HeroCartPlayer/PlayerCart.CartSlots` (`self.PlayerCartRef`))
    (bind _ascart_slot (cast `/Game/Blueprints/HeroCartPlayer/CartSlot` (`ChildActorComponent.ChildActor` _array_element)))
    (bind _assignedhero (`/Game/Blueprints/HeroCartPlayer/CartSlot.AssignedHero` _ascart_slot))
    ;[1 1 1] Add bonus if alive
    (if (`KismetSystemLibrary.IsValid` _assignedhero)
      (if (not (`/Game/Blueprints/Heroes/BaseHeroClass.IsAlive` _assignedhero))
        (bind _level (`/Game/Blueprints/Heroes/BaseHeroClass.Level` _assignedhero))
        (set `local.TempGold` (+ (* _level (`/Game/Blueprints/Heroes/BaseHeroClass.GoldPenaltyDead` _assignedhero)) (`local.TempGold`)))
        (set `local.TempXP` (+ (* _level (`/Game/Blueprints/Heroes/BaseHeroClass.XPBonusDead` _assignedhero)) (`local.TempXP`)))
        ;[1 1 1] Remove any dead heroes when doing the tally
        (`Actor.K2_DestroyActor` _assignedhero)
        (set `/Game/Blueprints/HeroCartPlayer/CartSlot.AssignedHero` null _ascart_slot))))
  (return (`local.TempGold`) (`local.TempXP`)))

(fn `GetMiscRoadBonus`
  (returns (Gold :type Integer) (XP :type Integer))
  (return 0 0))

(fn `GetVIPRoadBonus`
  (returns (Gold :type Integer) (XP :type Integer))
  (return 0 0))

(fn `GoTravel`
  ;[1 1 1] Set references to cart and clear selection if any
  (`/Engine/EditorBlueprintResources/StandardMacros.IsValid` (`self.PlayerCartRef`)
    (:`Is Valid`
      _)
    (:`Is Not Valid`
      (bind _asplayer_cart (cast `/Game/Blueprints/HeroCartPlayer/PlayerCart` (`GameplayStatics.GetPlayerPawn` 0)))
      (bind _output_get (set `self.PlayerCartRef` _asplayer_cart))))
  (`self.ClearHeroSelection`)
  ;[1 1 1] Create Level. TODO: Add overworld map stuff
  (`self.MakeRandomLevel` 1)
  ;[1 1 1] Set Player cart location
  (bind _ashero_cart_game_mode (cast `/Game/Blueprints/HeroCartGameMode` (`GameplayStatics.GetGameMode`)))
  (`Actor.K2_SetActorLocation` _output_get (`/Game/Blueprints/HeroCartGameMode.CartStartLocation` _ashero_cart_game_mode) false true)
  ;[1 1 1] Set active camera and mode
  (`ActorComponent.SetActive` (`/Game/Blueprints/HeroCartPlayer/PlayerCart.PlayCamera` _output_get) true false)
  (`ActorComponent.SetActive` (`/Game/Blueprints/HeroCartPlayer/PlayerCart.DioramaCam` _output_get) false false)
  (set `self.CurrentMode` "NewEnumerator2")
  (`/Game/Blueprints/HeroCartPlayer/PlayerCart.StartTravel` _output_get)
  ;[1 1 1] Clean diorama
  (`/Game/Blueprints/Environment/CartConfigDiorama.RemoveDiscardedHeroesAndDiorama` (`self.LastDioramaSpawned`))
  ;[1 1 1] Turn on the wall of death
  (`KismetMaterialLibrary.SetScalarParameterValue` "/Game/VFX/PostProcess/PostProcessGlobalParameters.PostProcessGlobalParameters" "WallOfDeathAlpha" 1.0))

(fn `MakeNewRandomHero`
  (params (Level :type Integer) (Tier :type Integer) (Transform :type "Transform Structure"))
  (returns (NewHero :type "/Game/Blueprints/Heroes/BaseHeroClass Object Reference"))
  (locals (TempNameList :type "Array of String"))
  (bind _outitem (`KismetArrayLibrary.Array_Random` (`local.TempNameList`)))
  ;[1 1 1] Get random class. TODO: Add class tiers
  (switch `/Game/Blueprints/BlueprintExtras/E_HeroClasses` (`KismetArrayLibrary.Array_Random` (`|MakeArray` "NewEnumerator0" "NewEnumerator3" "NewEnumerator11" :!type "/Game/Blueprints/BlueprintExtras/E_HeroClasses Enum"))
    (:`NewEnumerator0`
      (bind _returnvalue (`|SpawnActorFromClass` "/Game/Blueprints/Heroes/WarriorHero.WarriorHero_C" Transform "Undefined" "OverrideRootScale" null Level null))
      ;[1 1 1] Set a random name on new heroes. TODO: Add random attributes, equipment, etc.
      (set `/Game/Blueprints/Heroes/BaseHeroClass.HeroName` _outitem _returnvalue)
      (return _returnvalue))
    (:`NewEnumerator3`
      (bind _returnvalue_2 (`|SpawnActorFromClass` "/Game/Blueprints/Heroes/WitchHero.WitchHero_C" Transform "Undefined" "OverrideRootScale" null Level null))
      (set `/Game/Blueprints/Heroes/BaseHeroClass.HeroName` _outitem _returnvalue_2)
      (return _returnvalue_2))
    (:`NewEnumerator11`
      (bind _returnvalue_3 (`|SpawnActorFromClass` "/Game/Blueprints/Heroes/MerchantHero.MerchantHero_C" Transform "Undefined" "OverrideRootScale" null Level null))
      (set `/Game/Blueprints/Heroes/BaseHeroClass.HeroName` _outitem _returnvalue_3)
      (return _returnvalue_3))))

(fn `MakeNewTownHeroes`
  (bind _currenttown (`self.CurrentTown`))
  (for _index (range (`self.MaxTravelPostSlots`))
    (bind _output (`|GetArrayItem` (`/Game/Blueprints/Environment/Towns/TownBaseClass.CartSlotsInTP` _currenttown) _index))
    (bind _ascart_slot (cast `/Game/Blueprints/HeroCartPlayer/CartSlot` (`ChildActorComponent.ChildActor` _output)))
    (`/Engine/EditorBlueprintResources/StandardMacros.IsValid` (`/Game/Blueprints/HeroCartPlayer/CartSlot.AssignedHero` _ascart_slot)
      (:`Is Not Valid`
        (bind _newhero (`self.MakeNewRandomHero` (`/Game/Blueprints/Environment/Towns/TownBaseClass.TownLevel` _currenttown) (`/Game/Blueprints/Environment/Towns/TownBaseClass.TownTier` _currenttown) (`SceneComponent.K2_GetComponentToWorld` _output)))
        (`self.SetHeroSlot` _newhero _ascart_slot)))))

(fn `MakeRandomLevel`
  (params (ScalingLevel :type Integer) (Length :type Integer) (Biome :type "/Game/Blueprints/BlueprintExtras/LevelType Enum" :default "NewEnumerator0"))
  (locals (OffsetPerTile :type "Float (double-precision)" :default 8930.0) (CurrentOffset :type "Float (double-precision)") (GrasslandsStartTile :type "/Game/Blueprints/Environment/Tiles/TileBaseClass Class Reference" :default "BlueprintGeneratedClass'/Game/Blueprints/Environment/Tiles/Countryside_TileNormal_Start.Countryside_TileNormal_Start_C'") (GrasslandsEndTile :type "/Game/Blueprints/Environment/Tiles/TileBaseClass Class Reference" :default "BlueprintGeneratedClass'/Game/Blueprints/Environment/Tiles/Countryside_TileNormal_Ending.Countryside_TileNormal_Ending_C'") (GrassLandsMidTiles :type "Array of /Game/Blueprints/Environment/Tiles/TileBaseClass Class Reference"))
  (bind _leveltiles (`self.LevelTiles`))
  (`KismetArrayLibrary.Array_Clear` _leveltiles)
  (switch `/Game/Blueprints/BlueprintExtras/LevelType` Biome
    (:`NewEnumerator0`
      ;[1 1 1] Make start tile
      (bind _returnvalue (`|SpawnActorFromClass` (`local.GrasslandsStartTile`) (`KismetMathLibrary.MakeTransform` (0.0 0.0 0.0)) "Undefined" "OverrideRootScale" null null))
      (set `/Game/Blueprints/Environment/Tiles/TileBaseClass.ScalingLevel` ScalingLevel _returnvalue)
      (set `local.CurrentOffset` (`local.OffsetPerTile`))
      (`KismetArrayLibrary.Array_Add` _leveltiles _returnvalue)
      ;[1 1 1] Create mid tiles
      (for _ (range Length)
        (bind _returnvalue_2 (`|SpawnActorFromClass` (`KismetArrayLibrary.Array_Random` (`local.GrassLandsMidTiles`)) (`KismetMathLibrary.MakeTransform` (`KismetMathLibrary.MakeVector` (`local.CurrentOffset`))) "Undefined" "OverrideRootScale" null null))
        (set `local.CurrentOffset` (+ (`local.CurrentOffset`) (`local.OffsetPerTile`)))
        (set `/Game/Blueprints/Environment/Tiles/TileBaseClass.ScalingLevel` ScalingLevel _returnvalue_2)
        (`KismetArrayLibrary.Array_Add` _leveltiles _returnvalue_2))
      ;[1 1 1] Make end tile
      (bind _returnvalue_3 (`|SpawnActorFromClass` (`local.GrasslandsEndTile`) (`KismetMathLibrary.MakeTransform` (`KismetMathLibrary.MakeVector` (`local.CurrentOffset`))) "Undefined" "OverrideRootScale" null null))
      (set `/Game/Blueprints/Environment/Tiles/TileBaseClass.ScalingLevel` ScalingLevel _returnvalue_3)
      (`KismetArrayLibrary.Array_Add` _leveltiles _returnvalue_3))))

(fn `MoveCartHeroesToTownSlots`
  (locals (CurrentSlotToFill :type Integer))
  (bind _currentslottofill (`local.CurrentSlotToFill`))
  (for _array_element (`/Game/Blueprints/HeroCartPlayer/PlayerCart.CartSlots` (`self.PlayerCartRef`))
    (bind _ascart_slot (cast `/Game/Blueprints/HeroCartPlayer/CartSlot` (`ChildActorComponent.ChildActor` _array_element)))
    (bind _assignedhero (`/Game/Blueprints/HeroCartPlayer/CartSlot.AssignedHero` _ascart_slot))
    (`/Engine/EditorBlueprintResources/StandardMacros.IsValid` _assignedhero
      (:`Is Valid`
        (bind _ascart_slot_2 (cast `/Game/Blueprints/HeroCartPlayer/CartSlot` (`ChildActorComponent.ChildActor` (`|GetArrayItem` (`/Game/Blueprints/Environment/Towns/TownBaseClass.CartSlotsInTP` (`self.CurrentTown`)) _currentslottofill))))
        (`self.SetHeroSlot` _assignedhero _ascart_slot_2 true)
        (`/Engine/EditorBlueprintResources/StandardMacros.IncrementInt` _currentslottofill)))))

(fn `Remove Enemy from List`
  (params (EnemyRef :type "/Game/Blueprints/Enemies/BaseEnemyClass Object Reference"))
  (bind _spawnedenemies (`self.SpawnedEnemies`))
  (`KismetArrayLibrary.Array_Remove` _spawnedenemies (`KismetArrayLibrary.Array_Find` _spawnedenemies EnemyRef)))

(fn `SelectHeroToEdit`
  (params (HeroRef :type "/Game/Blueprints/Heroes/BaseHeroClass Object Reference"))
  (bind _selectedhero (`self.SelectedHero`))
  (`/Engine/EditorBlueprintResources/StandardMacros.IsValid` HeroRef
    (:`Is Valid`
      (if (== _selectedhero HeroRef)
        ;[1 1 1] Remove selection and disable FOV display
        (`/Engine/EditorBlueprintResources/StandardMacros.IsValid` _selectedhero
          (:`Is Valid`
            (`SceneComponent.SetVisibility` (`/Game/Blueprints/Heroes/BaseHeroClass.Plane` _selectedhero) false true))
          (:`Is Not Valid`
            _))
        (set `self.SelectedHero` null)
        (else
          ;[1 1 1] Select hero and show FOV display
          (`/Engine/EditorBlueprintResources/StandardMacros.IsValid` _selectedhero
            (:`Is Valid`
              (`SceneComponent.SetVisibility` (`/Game/Blueprints/Heroes/BaseHeroClass.Plane` _selectedhero) false true))
            (:`Is Not Valid`
              _))
          (bind _output_get (set `self.SelectedHero` HeroRef))
          (`SceneComponent.SetVisibility` (`/Game/Blueprints/Heroes/BaseHeroClass.Plane` _output_get) true true))))))

(fn `SetHeroSlot`
  (params (TargetHero :type "/Game/Blueprints/Heroes/BaseHeroClass Object Reference") (TargetSlot :type "/Game/Blueprints/HeroCartPlayer/CartSlot Object Reference") (ClearOldSlot :type Boolean))
  ;[1 1 1] Set New location to slot position
  (`Actor.K2_SetActorLocation` TargetHero (`SceneComponent.K2_GetComponentLocation` (`/Game/Blueprints/HeroCartPlayer/CartSlot.DefaultSceneRoot` TargetSlot)) false true)
  ;[1 1 1] Set new hero ref on slot and reparent hero
  (`Actor.K2_AttachToActor` TargetHero TargetSlot "None" "KeepWorld" "KeepWorld" "KeepWorld" true)
  (set `/Game/Blueprints/HeroCartPlayer/CartSlot.AssignedHero` TargetHero TargetSlot)
  ;[1 1 1] Clear hero ref on old slot if needed
  (if ClearOldSlot
    (set `/Game/Blueprints/HeroCartPlayer/CartSlot.AssignedHero` null (`/Game/Blueprints/Heroes/BaseHeroClass.AttachedToSlot` TargetHero)))
  (set `/Game/Blueprints/Heroes/BaseHeroClass.AttachedToSlot` TargetSlot TargetHero)
  (return))

(fn `SetUpConfigDiorama`
  (bind _playercartref (`self.PlayerCartRef`))
  ;[1 1 1] Spawn the diorama actor and fill up its slots with new random heroes
  (`/Engine/EditorBlueprintResources/StandardMacros.IsValid` _playercartref
    (:`Is Valid`
      (bind _returnvalue (`|SpawnActorFromClass` "/Game/Blueprints/Environment/CartConfigDiorama.CartConfigDiorama_C" (`KismetMathLibrary.MakeTransform` (- (.location (`Actor.GetTransform` _playercartref)) (130.0 300.0 70.0)) (`KismetMathLibrary.ComposeRotators` (.rotation (`Actor.GetTransform` _playercartref)) (struct :`Yaw` -15.0)) (0.75 0.75 0.25)) "Undefined" "OverrideRootScale" null null))
      (`/Game/Blueprints/Environment/CartConfigDiorama.FillSlotsWithRandomHeroes` _returnvalue self)
      (set `self.LastDioramaSpawned` _returnvalue))))

(fn `SetupTown`
  (locals (TownNames :type "Array of String"))
  (bind _returnvalue (`|SpawnActorFromClass` "/Game/Blueprints/Environment/Towns/TownBaseClass.TownBaseClass_C" (`KismetMathLibrary.Conv_VectorToTransform` (- (`Actor.K2_GetActorLocation` (`self.PlayerCartRef`)) (3000.0 -550.0 -20.0))) "Undefined" "OverrideRootScale" null (`KismetArrayLibrary.Array_Random` (`local.TownNames`)) (`self.MaxTravelPostSlots`) null))
  (set `self.CurrentTown` _returnvalue)
  (`self.MoveCartHeroesToTownSlots`)
  (`self.MakeNewTownHeroes`))

(fn `StartInitialCartConfigMode`
  ;[1 1 1] Set player cart reference
  (`/Engine/EditorBlueprintResources/StandardMacros.IsValid` (`self.PlayerCartRef`)
    (:`Is Valid`
      _)
    (:`Is Not Valid`
      (bind _asplayer_cart (cast `/Game/Blueprints/HeroCartPlayer/PlayerCart` (`GameplayStatics.GetPlayerPawn` 0)))
      (bind _output_get (set `self.PlayerCartRef` _asplayer_cart))))
  ;[1 1 1] Set Edit camera
  (`ActorComponent.SetActive` (`/Game/Blueprints/HeroCartPlayer/PlayerCart.PlayCamera` _output_get) false false)
  (`ActorComponent.SetActive` (`/Game/Blueprints/HeroCartPlayer/PlayerCart.DioramaCam` _output_get) true false)
  ;[1 1 1] Set up the cart config 3D actor
  (set `self.CurrentMode` "NewEnumerator1")
  (`self.SetUpConfigDiorama`)
  (set `self.IsMainHUDVisible` true))